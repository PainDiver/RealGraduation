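; GoalPoint_BP is the finish-line actor that ends the level when an actor overlaps it.
; On authority it sets a new BP_GoodSky preset and effect, then notifies the overlapping MyCharacter_BP's MyWorldTimer_BP controller of the arrival.
; Authority (after those casts succeed) and remotes (on any overlap) share a 25-second delay, then remove all widgets and call MyServerTravel on the game instance to ScoreMap as a listen server.
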(event Custom|ServerWeatherChange
  (bind _returnvalue (Actor|GetActorOfClass "/Game/GoodSky/Blueprint/BP_GoodSky.BP_GoodSky_C"))
  (Variables|/Game/GoodSky/Blueprint/BP_GoodSky.BP_GoodSky_C|SetSkyPreset _returnvalue "NewEnumerator13")
  (Variables|/Game/GoodSky/Blueprint/BP_GoodSky.BP_GoodSky_C|SetSkyEffect _returnvalue "NewEnumerator2"))

(event EventBeginPlay)

(event Collision|EventActorBeginOverlap
  (params (OtherActor :type Actor%20Object%20Reference))
  (Networking|SwitchHasAuthority
    (:Authority
      (CallFunction|ServerWeatherChange)
      (bind _asmy_character_bp (Utilities|Casting|CastToMyCharacter_BP OtherActor))
      (bind _asmy_world_timer_bp (Utilities|Casting|CastToMyWorldTimer_BP (Pawn|GetController _asmy_character_bp)))
      (Class|MyWorldTimer|NotifyArrival _asmy_world_timer_bp))
    (:Remote
      _))
  (Utilities|FlowControl|Delay 25.0)
  (Viewport|RemoveAllWidgets)
  (bind _asmy_game_instance_bp (Utilities|Casting|CastToMyGameInstance_BP (Game|GetGameInstance)))
  (Class|MyGameInstance|MyServerTravel _asmy_game_instance_bp "/Game/map/ScoreMap" "/Game/ScoreMap/MyScoreMapGameMode_BP.MyScoreMapGameMode_BP_C?listen" true))

(event EventTick
  (params (DeltaSeconds :type Float%20%28single-precision%29)))

(fn ConstructionScript)