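; Player state Blueprint that stores a player's ready state, selected map and travel signal, and moves the player to a dedicated server.
; A looping timer started on BeginPlay polls the travel signal.
; When signaled, it clears the signal and, if a server URL is set, stops polling and disables input.
; After a short delay, it runs an "Open steam." console command with that URL appended.
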(event Custom|SetReady
  (params (NewParam :type Boolean))
  (Variables|Default|SetIsReady NewParam))

(event Custom|SelectMap
  (params (NewParam :type String))
  (Variables|Default|SetSelectedMap NewParam))

(event Custom|WaitForSignal
  (if (Variables|Default|GetSignalToTravel)
    (CallFunction|SetSignal false)
    (if (not (Utilities|Array|IsEmpty (Variables|Default|GetDediURL)))
      (Utilities|Time|ClearandInvalidateTimerbyHandle (Variables|Default|GetTimer))
      (Input|DisableInput (Game|GetPlayerController 0))
      (Utilities|FlowControl|Delay 2.0)
      (Development|ExecuteConsoleCommand (Utilities|String|Append (Utilities|String|MakeLiteralString "Open steam.") (Variables|Default|GetDediURL)) 0))
    (else
      (Development|PrintString "SignalCheck"))))

(event Custom|SetSignal
  (params (NewParam :type Boolean))
  (Variables|Default|SetSignalToTravel NewParam))

(event EventBeginPlay
  (bind _returnvalue (Utilities|Time|SetTimerbyEvent (delegate Custom|WaitForSignal) 2.0 true))
  (Variables|Default|SetTimer _returnvalue))

(event EventTick
  (params (DeltaSeconds :type Float%20%28single-precision%29)))

(fn ConstructionScript)