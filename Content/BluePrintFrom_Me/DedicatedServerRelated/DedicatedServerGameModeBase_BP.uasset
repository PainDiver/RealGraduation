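; Game mode for TwistRun dedicated servers, which registers a session and acts as either master matchmaker or map server.
; Non-master servers travel to the Waikiki or Space Station ready map chosen by the game instance.
; The master spawns servers and, on a looping timer, refreshes server info and queues ready players by selected map.
; Queued players receive a travel signal and server URL through PlayerState; without an open server, another is spawned.
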(event Custom|CollectGamers
  (bind _returnvalue (Game|GetGameInstance))
  (bind _asmy_game_instance_bp (Utilities|Casting|CastToMyGameInstance_BP _returnvalue))
  (Class|MyGameInstance|ReadAllDedicatedServerInfo _asmy_game_instance_bp)
  (Utilities|FlowControl|Delay 5.0)
  (bind _returnvalue_2 (Class|MyGameInstance|GetEnterableWaikikiDediServer _asmy_game_instance_bp))
  (bind _outactors (Actor|GetAllActorsOfClass "/Game/BluePrintFrom_Me/Player/MyCharacter_BP.MyCharacter_BP_C"))
  (bind _array_element (Utilities|Array|ForEachLoopwithBreak _outactors)
    (:LoopBody
      (Utilities|IsValid (.AsMy%20Player%20State%20BP (Utilities|Casting|CastToMyPlayerState_BP (Variables|/Script/Engine.Pawn|GetPlayerState _array_element)))
        (:Is%20Valid
          (if (Variables|/Game/BluePrintFrom_Me/MyPlayerState_BP.MyPlayerState_BP_C|GetIsReady (.AsMy%20Player%20State%20BP (Utilities|Casting|CastToMyPlayerState_BP (Variables|/Script/Engine.Pawn|GetPlayerState _array_element))))
            (switch string (Variables|/Game/BluePrintFrom_Me/MyPlayerState_BP.MyPlayerState_BP_C|GetSelectedMap (.AsMy%20Player%20State%20BP (Utilities|Casting|CastToMyPlayerState_BP (Variables|/Script/Engine.Pawn|GetPlayerState _array_element))))
              (:Default
                (Utilities|Array|AddUnique (Variables|Default|GetWaikikiQueue) _array_element :!label _label))
              (:Waikiki
                (goto _label))
              (:SpaceStation
                (Utilities|Array|AddUnique (Variables|Default|GetSpaceStationQueue) _array_element)))
            (else
              (Development|PrintString "Not Ready")
              (Utilities|Array|RemoveItem (Variables|Default|GetWaikikiQueue) _array_element)
              (Utilities|Array|RemoveItem (Variables|Default|GetSpaceStationQueue) _array_element))))
        (:Is%20Not%20Valid
          (Development|PrintString "State not Valid"))))
    (:Completed
      (CallFunction|SendReadPlayers))))

(event Custom|SendReadPlayers
  (bind _returnvalue (Game|GetGameInstance))
  (bind _asmy_game_instance_bp (Utilities|Casting|CastToMyGameInstance_BP _returnvalue))
  (Development|PrintString (Utilities|String|Append (Utilities|String|ToString(Integer) (Utilities|Array|Length (Variables|Default|GetWaikikiQueue))) " wating for Wakiki"))
  (Development|PrintString (Utilities|String|Append (Utilities|String|ToString(Integer) (Utilities|Array|Length (Variables|Default|GetSpaceStationQueue))) " wating for SpaceStation"))
  (Utilities|FlowControl|Sequence
    (:then_0
      (if (>= (Utilities|Array|Length (Variables|Default|GetWaikikiQueue)) 1)
        (if (not (Variables|Default|Getpending))
          (Variables|Default|Setpending true)
          (Development|PrintString "Open OtherMap")
          (bind _returnvalue_2 (Class|MyGameInstance|GetEnterableWaikikiDediServer _asmy_game_instance_bp))
          (Development|PrintString (Utilities|String|Append _returnvalue_2 " is Enterable"))
          (if (Utilities|Enum|NotEqual(Enum) _returnvalue_2 "Default")
            (bind _array_element (Utilities|Array|ForEachLoopwithBreak (Variables|Default|GetWaikikiQueue))
              (:LoopBody
                (Utilities|IsValid _array_element
                  (:Is%20Valid
                    (Variables|/Game/BluePrintFrom_Me/MyPlayerState_BP.MyPlayerState_BP_C|SetIsReady (.AsMy%20Player%20State%20BP (Utilities|Casting|CastToMyPlayerState_BP (Variables|/Script/Engine.Pawn|GetPlayerState _array_element))) false)
                    (Variables|/Game/BluePrintFrom_Me/MyPlayerState_BP.MyPlayerState_BP_C|SetSignalToTravel (.AsMy%20Player%20State%20BP (Utilities|Casting|CastToMyPlayerState_BP (Variables|/Script/Engine.Pawn|GetPlayerState _array_element))) true)
                    (Variables|/Game/BluePrintFrom_Me/MyPlayerState_BP.MyPlayerState_BP_C|SetDediURL (.AsMy%20Player%20State%20BP (Utilities|Casting|CastToMyPlayerState_BP (Variables|/Script/Engine.Pawn|GetPlayerState _array_element))) _returnvalue_2)
                    (Utilities|Array|RemoveItem (Variables|Default|GetWaikikiQueue) _array_element)
                    (Variables|Default|Setpending false)))))
            (else
              (Class|MyGameInstance|CreateDedicatedServers _asmy_game_instance_bp)
              (Variables|Default|Setpending false))))))
    (:then_1
      (if (>= (Utilities|Array|Length (Variables|Default|GetSpaceStationQueue)) 1)
        (if (not (Variables|Default|Getpending))
          (Variables|Default|Setpending true)
          (bind _returnvalue_3 (Class|MyGameInstance|GetEnterableSpacestationDediServer _asmy_game_instance_bp))
          (Development|PrintString (Utilities|String|Append _returnvalue_3 "is Enterable"))
          (if (Utilities|Enum|NotEqual(Enum) _returnvalue_3 "Default")
            (bind _array_element_2 (Utilities|Array|ForEachLoopwithBreak (Variables|Default|GetSpaceStationQueue))
              (:LoopBody
                (Utilities|IsValid _array_element_2
                  (:Is%20Valid
                    (Variables|/Game/BluePrintFrom_Me/MyPlayerState_BP.MyPlayerState_BP_C|SetIsReady (.AsMy%20Player%20State%20BP (Utilities|Casting|CastToMyPlayerState_BP (Variables|/Script/Engine.Pawn|GetPlayerState _array_element_2))) false)
                    (Variables|/Game/BluePrintFrom_Me/MyPlayerState_BP.MyPlayerState_BP_C|SetSignalToTravel (.AsMy%20Player%20State%20BP (Utilities|Casting|CastToMyPlayerState_BP (Variables|/Script/Engine.Pawn|GetPlayerState _array_element_2))) true)
                    (Variables|/Game/BluePrintFrom_Me/MyPlayerState_BP.MyPlayerState_BP_C|SetDediURL (.AsMy%20Player%20State%20BP (Utilities|Casting|CastToMyPlayerState_BP (Variables|/Script/Engine.Pawn|GetPlayerState _array_element_2))) _returnvalue_3)
                    (Utilities|Array|RemoveItem (Variables|Default|GetSpaceStationQueue) _array_element_2)
                    (Variables|Default|Setpending false)))))
            (else
              (Class|MyGameInstance|CreateDedicatedServers _asmy_game_instance_bp)
              (Variables|Default|Setpending false))))))))

(event EventBeginPlay
  (bind _returnvalue (Game|GetGameInstance))
  (bind _asmy_game_instance_bp (Utilities|Casting|CastToMyGameInstance_BP _returnvalue))
  (if (Networking|IsServer)
    (Utilities|FlowControl|Delay 1.0)
    (Class|MyGameInstance|InitializeBranch (.AsMy%20Game%20Instance%20BP (Utilities|Casting|CastToMyGameInstance_BP (Game|GetGameInstance))) (Utilities|String|MakeLiteralString "http://211.34.239.132 
:8335/"))
    (Utilities|FlowControl|Delay 3.0)
    (|AdvancedSession (Utilities|Array|MakeArray (Class|AdvancedSessionsLibrary|MakeLiteralSessionPropertyString "ServerName" "TwistRun")) (Game|GetPlayerController 0) 100 0 false true true false false false false true false true
      (:OnSuccess
        (if (Variables|/Script/MyProject4.MyGameInstance|Get_bIsMasterServer (.AsMy%20Game%20Instance%20BP (Utilities|Casting|CastToMyGameInstance_BP (Game|GetGameInstance))))
          (Class|MyGameInstance|LogOutMasterServer _asmy_game_instance_bp)
          (Class|MyGameInstance|CreateDedicatedServers _asmy_game_instance_bp)
          (Utilities|FlowControl|Delay 0.5)
          (Class|MyGameInstance|CreateDedicatedServers _asmy_game_instance_bp)
          (Development|PrintString (Utilities|String|Append "Dedi Suc:" (Class|AdvancedSessionsLibrary|GetCurrentSessionIDasString)))
          (Class|MyGameInstance|WriteMasterServerInfo _asmy_game_instance_bp (Class|AdvancedSessionsLibrary|GetCurrentSessionIDasString))
          (Utilities|Time|SetTimerbyEvent (delegate Custom|CollectGamers) 1e+01 true)
          (else
            (bind _returnvalue_2 (Class|MyGameInstance|BranchMap _asmy_game_instance_bp))
            (switch Utilities|FlowControl|Switch|SwitchonEMapSelection _returnvalue_2
              (:EMS_Waikiki
                (Development|PrintString "Branch to Waikiki")
                (Development|ExecuteConsoleCommand "ServerTravel/Game/map/ReadyMap?game=/Game/ReadyRoomMap/MyReadyRoomGameModeBase_BP.MyReadyRoomGameModeBase_BP_C" 0))
              (:EMS_SpaceStation
                (Development|PrintString "Branch to Space Station")
                (Development|ExecuteConsoleCommand "ServerTravel/Game/map/SpaceStationReadyMap?game=/Game/ReadyRoomMap/MyReadyRoomGameModeBase_BP.MyReadyRoomGameModeBase_BP_C" 0))))))
      (:OnFailure
        (Development|PrintString "Dedi fail")))))

(event EventTick
  (params (DeltaSeconds :type Float%20%28single-precision%29)))

(event EventOnLogout
  (params (ExitingController :type Controller%20Object%20Reference))
  (Development|PrintString "SomeonLoggedOut")
  (Class|MyGameInstance|LinkMasterServerInfo (.AsMy%20Game%20Instance%20BP (Utilities|Casting|CastToMyGameInstance_BP (Game|GetGameInstance))) false))

(event EventPostLogin
  (params (NewPlayer :type Player%20Controller%20Object%20Reference)))

(fn ConstructionScript)