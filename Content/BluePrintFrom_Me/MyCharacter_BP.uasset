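; Player character Blueprint that handles name tags, a crosshair and an options menu.
; On begin play, the locally controlled character creates both widgets, passes the GameInstance character name to ServerNameSet, and marks its own tag with a green star.
; Non-local copies poll on a delay loop until that name is filled, then show it on the tag.
; The Option input adds the menu to the viewport or toggles its visibility.
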(event Custom|ServerNameSet
  (params (NewParam :type Text))
  (Variables|Default|SetCharacterNameFromInstance NewParam))

(event EventBeginPlay
  (bind _returnvalue (Game|GetPlayerController 0))
  (bind _characternamefrominstance (Variables|Default|GetCharacterNameFromInstance))
  (if (Pawn|IsLocallyControlled)
    (bind _returnvalue_2 (UserInterface|CreateWidget "/Game/HUD/Crosshair_UI.Crosshair_UI_C" _returnvalue))
    (UserInterface|Viewport|AddtoViewport _returnvalue_2 0)
    (bind _returnvalue_3 (UserInterface|CreateWidget "/Game/HUD/Option_UI.Option_UI_C" _returnvalue))
    (Variables|Default|Setoption _returnvalue_3)
    (bind _asmy_game_instance_bp (Utilities|Casting|CastToMyGameInstance_BP (Game|GetGameInstance)))
    (CallFunction|ServerNameSet (Utilities|Text|ToText(String) (._CharacterName (Utilities|Struct|BreakCharacterInfo (Variables|/Script/MyProject4.MyGameInstance|Get_characterInfo _asmy_game_instance_bp)))))
    (bind _asname_tag_ui (Utilities|Casting|CastToNameTag_UI (UserInterface|GetUserWidgetObject (Variables|Default|GetNameTag))))
    (Appearance|SetColorandOpacity (Variables|/Game/HUD/NameTag_UI.NameTag_UI_C|GetName _asname_tag_ui) (Utilities|Struct|MakeSlateColor "(R=0.238189,G=1.000000,B=0.000000,A=1.000000)") :!class /Script/UMG.TextBlock)
    (Rendering|Components|TextRender|SetText (Variables|/Game/HUD/NameTag_UI.NameTag_UI_C|GetName _asname_tag_ui) "★")
    (else
      (Utilities|FlowControl|Delay 0.5 :!label _label)
      (bind _asname_tag_ui_2 (Utilities|Casting|CastToNameTag_UI (UserInterface|GetUserWidgetObject (Variables|Default|GetNameTag))))
      (if (Utilities|Text|TextIsEmpty _characternamefrominstance)
        (goto _label)
        (else
          (bind _output_get (Variables|/Game/HUD/NameTag_UI.NameTag_UI_C|Setcharactername _asname_tag_ui_2 _characternamefrominstance))
          (Rendering|Components|TextRender|SetText (Variables|/Game/HUD/NameTag_UI.NameTag_UI_C|GetName _asname_tag_ui_2) _output_get))))))

(event Collision|EventActorBeginOverlap
  (params (OtherActor :type Actor%20Object%20Reference)))

(event Input|ActionEvents|InputActionOption
  (params (Key :type Key%20Structure :default "None"))
  (bind _option (Variables|Default|Getoption))
  (:Pressed
    (Utilities|IsValid _option
      (:Is%20Valid
        (switch Utilities|FlowControl|Switch|SwitchonESlateVisibility (Widget|GetVisibility _option)
          (:Visible
            (if (UserInterface|Viewport|IsinViewport _option)
              (Widget|SetVisibility _option "Hidden")
              (else
                (UserInterface|Viewport|AddtoViewport _option 0))))
          (:Hidden
            (Widget|SetVisibility _option "Visible")))))))

(fn ConstructionScript)