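; Laser beam actor, apparently for a laser turret, that kills and respawns the player character on hit.
; ShootLaser line-traces to the target, sets the Niagara beam end and places or hides spark and hit effects.
; The first character hit triggers a DoOnce sequence: zero gravity, disabled input, ragdoll and material dissolve, then restoration and a ReplicatorComponent respawn after a delay.
; StopLaser scales the beam by timeline and deactivates the effects.
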(event Custom|FadeIn
  (bind _character (Variables|Default|GetCharacter))
  (bind _mesh (Variables|/Script/Engine.Character|GetMesh _character))
  (bind _returnvalue (Rendering|Material|CreateDynamicMaterialInstance _mesh 0 (Rendering|Material|GetMaterial _mesh 0) "None" :!class /Script/Engine.PrimitiveComponent))
  (bind (_direction _dissolve _const) (Timeline|FadeInTimeline PlayFromStart)
    (:Update
      (Utilities|FlowControl|Sequence
        (:then_0
          (Rendering|Material|SetScalarParameterValue _returnvalue "DissolveParam" _dissolve :!class /Script/Engine.MaterialInstanceDynamic))
        (:then_1
          (Rendering|Material|SetScalarParameterValue _returnvalue "ConstParam2" _const :!class /Script/Engine.MaterialInstanceDynamic))))))

(event Custom|UnRagdoll
  (bind _character (Variables|Default|GetCharacter))
  (bind _mesh (Variables|/Script/Engine.Character|GetMesh _character))
  (Transformation|AttachComponentToComponent _mesh (Variables|/Script/Engine.Character|GetCapsuleComponent _character) "None" "SnapToTarget" "SnapToTarget" "KeepWorld" true)
  (Physics|SetSimulatePhysics _mesh false)
  (Components|MoveComponentTo (Variables|/Script/MyProject4.MyCharacter|Get_springArm _character) "0, 0,60.000000" "0, 0, 0" false false 0.0 false))

(event Custom|DisableGravity
  (Variables|/Script/Engine.CharacterMovementComponent|SetGravityScale (Variables|/Script/Engine.Character|GetCharacterMovement (Variables|Default|GetCharacter)) 0.0))

(event Custom|DisableController
  (Input|DisableInput (Variables|Default|GetCharacter) 0))

(event Custom|Ragdoll
  (Physics|SetSimulatePhysics (Variables|/Script/Engine.Character|GetMesh (Variables|Default|GetCharacter)) true))

(event Custom|EnableCollision
  (Collision|SetCollisionEnabled (Variables|/Script/Engine.Character|GetCapsuleComponent (Variables|Default|GetCharacter)) "QueryAndPhysics"))

(event Custom|FadeOut
  (bind _character (Variables|Default|GetCharacter))
  (bind _mesh (Variables|/Script/Engine.Character|GetMesh _character))
  (bind _returnvalue (Rendering|Material|CreateDynamicMaterialInstance _mesh 0 (Rendering|Material|GetMaterial _mesh 0) "None" :!class /Script/Engine.PrimitiveComponent))
  (bind (_direction _dissolve _const) (Timeline|FadeOutTimeline PlayFromStart)
    (:Update
      (Utilities|FlowControl|Sequence
        (:then_0
          (Rendering|Material|SetScalarParameterValue _returnvalue "DissolveParam" _dissolve :!class /Script/Engine.MaterialInstanceDynamic))
        (:then_1
          (Rendering|Material|SetScalarParameterValue _returnvalue "ConstParam2" _const :!class /Script/Engine.MaterialInstanceDynamic))))))

(event Custom|ShootLaser
  (params (StartLocation :type Vector) (TargetLocation :type Vector))
  (bind _laser_hit_niagara (Variables|Default|GetLaser%20Hit%20Niagara))
  (bind _laser_niagara (Variables|Default|GetLaser%20Niagara))
  (bind _laser_spark_niagara (Variables|Default|GetLaser%20Spark%20Niagara))
  (bind _outhit (Collision|LineTraceByChannel StartLocation TargetLocation "TraceTypeQuery2" false 0 "ForDuration"))
  (Effects|Components|ParticleSystem|SetVectorParameter _laser_niagara "User.BeamEnd" (Math|Vector|SelectVector (.Location (Collision|BreakHitResult _outhit)) (.TraceEnd (Collision|BreakHitResult _outhit)) (Utilities|IsValid (.HitActor (Collision|BreakHitResult _outhit)))))
  (Effects|Components|ParticleSystem|SetFloatParameter _laser_niagara "User.Scale" 4.0)
  (Utilities|FlowControl|Sequence
    (:then_0
      (if (Utilities|IsValid (.HitActor (Collision|BreakHitResult _outhit)))
        (Transformation|SetWorldLocation _laser_spark_niagara (Math|Vector|SelectVector (.Location (Collision|BreakHitResult _outhit)) (.TraceEnd (Collision|BreakHitResult _outhit)) (Utilities|IsValid (.HitActor (Collision|BreakHitResult _outhit)))) false false)
        (Transformation|SetWorldRotation _laser_spark_niagara (Math|Conversions|RotationFromXVector (* "0, 0, 0" -1)) false false)
        (Effects|Components|ParticleSystem|SetFloatParameter _laser_spark_niagara "User.Scale" 1.0)
        (Transformation|SetWorldLocation _laser_hit_niagara (Math|Vector|SelectVector (.Location (Collision|BreakHitResult _outhit)) (.TraceEnd (Collision|BreakHitResult _outhit)) (Utilities|IsValid (.HitActor (Collision|BreakHitResult _outhit)))) false false)
        (Effects|Components|ParticleSystem|SetFloatParameter _laser_hit_niagara "User.Scale" 1.0)
        (else
          (Effects|Components|ParticleSystem|SetFloatParameter _laser_spark_niagara "User.Scale" 0.0)
          (Effects|Components|ParticleSystem|SetFloatParameter _laser_hit_niagara "User.Scale" 0.0))))
    (:then_1
      (if (.bSuccess (Utilities|Casting|CastToMyCharacter_BP (.HitActor (Collision|BreakHitResult _outhit))))
        (Variables|Default|SetCharacter (.AsMy%20Character%20BP (Utilities|Casting|CastToMyCharacter_BP (.HitActor (Collision|BreakHitResult _outhit)))))
        (Utilities|FlowControl|DoOnce false
          (:Completed
            (CallFunction|DisableGravity)
            (CallFunction|FadeOut)
            (CallFunction|DisableController)
            (CallFunction|Ragdoll)
            (Utilities|FlowControl|Delay 2.5)
            (CallFunction|UnRagdoll)
            (CallFunction|Fadein)
            (CallFunction|EnableGravity)
            (Class|MyCharacterReplicatorComponent|Respawn (Variables|/Script/MyProject4.MyCharacter|Get_replicatorComponent (Variables|Default|GetCharacter)))
            (CallFunction|EnableController)))))))

(event Custom|EnableGravity
  (Variables|/Script/Engine.CharacterMovementComponent|SetGravityScale (Variables|/Script/Engine.Character|GetCharacterMovement (Variables|Default|GetCharacter)) 1.0))

(event Custom|StopLaser
  (bind _laser_niagara (Variables|Default|GetLaser%20Niagara))
  (bind _laser_hit_niagara (Variables|Default|GetLaser%20Hit%20Niagara))
  (bind _laser_spark_niagara (Variables|Default|GetLaser%20Spark%20Niagara))
  (bind _scale (Timeline|StopLaserTimeline Play)
    (:Update
      (Effects|Components|ParticleSystem|SetFloatParameter _laser_niagara "User.Scale" _scale)
      (Effects|Components|ParticleSystem|SetFloatParameter _laser_spark_niagara "User.Scale" 0.0)
      (Effects|Components|ParticleSystem|SetFloatParameter _laser_hit_niagara "User.Scale" 0.0)
      (Utilities|FlowControl|Delay 1.75)
      (Utilities|FlowControl|Sequence
        (:then_0
          (Components|Activation|Deactivate _laser_spark_niagara))
        (:then_1
          (Components|Activation|Deactivate _laser_hit_niagara))
        (:then_2
          (Components|Activation|Deactivate _laser_niagara))))))

(event Custom|SpeedDown
  (bind _character (Variables|Default|GetCharacter))
  (bind _mesh (Variables|/Script/Engine.Character|GetMesh _character))
  (Transformation|SetWorldLocation (Variables|/Script/Engine.Character|GetCapsuleComponent _character) (Transformation|GetSocketLocation _mesh "upper") false false)
  (Physics|SetPhysicsLinearVelocity _mesh (Math|Interpolation|VInterpTo (Transformation|GetComponentVelocity _mesh) "0, 0, 0" (Utilities|Time|GetWorldDeltaSeconds) 25.0) false "None"))

(event Custom|DisableCollision
  (Collision|SetCollisionEnabled (Variables|/Script/Engine.Character|GetCapsuleComponent (Variables|Default|GetCharacter)) "NoCollision"))

(event Custom|EnableController
  (Input|EnableInput (Variables|Default|GetCharacter) 0))

(fn ConstructionScript)