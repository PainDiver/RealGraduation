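; Laser turret actor that runs a looping timed attack cycle: spread, charge, fire along its forward axis, then fold.
; Timelines animate the wings, core roll and recoil-like core slide, and scale the charging Niagara effect.
; OnOffLaser toggles Tick, which spawns and attaches a CD_LaserTurret_Laser_BP when none exists and updates its endpoints each frame.
; Stopping the laser destroys that actor after a delay.
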(event Custom|ShootLaser
  (bind _laser (Variables|Default|GetLaser))
  (bind _returnvalue (Transformation|GetWorldLocation _laser))
  (Utilities|IsValid (Variables|Default|GetSpawnedLaser)
    (:Is%20Valid
      (if (Variables|Default|GetIsShooting?)
        (Default|ShootLaser (Variables|Default|GetSpawnedLaser) _returnvalue (+ _returnvalue (* (Math|Rotator|GetRotationXVector (Transformation|GetWorldRotation _laser)) (Variables|Default|GetRange))) :!label _label)))
    (:Is%20Not%20Valid
      (Audio|PlaySoundatLocation 0 (Transformation|GetWorldLocation (Variables|Default|GetCore)) "0, 0, 0" 1.5 0.3 0.1 0 0 0)
      (bind _returnvalue_2 (Game|SpawnActorfromClass "/Game/BluePrintFrom_Me/CD_LaserTurret/CD_LaserTurret_Laser_BP.CD_LaserTurret_Laser_BP_C" (Math|Transform|MakeTransform "0, 0, 0" "0, 0, 0" "1,1,1") "Undefined" self 0))
      (bind _output_get (Variables|Default|SetSpawnedLaser _returnvalue_2))
      (Transformation|AttachComponentToComponent _output_get (Variables|Default|GetLaser) "None" "SnapToTarget" "SnapToTarget" "KeepRelative" true)
      (goto _label))))

(event Custom|StopLaser
  (bind _spawnedlaser (Variables|Default|GetSpawnedLaser))
  (Utilities|IsValid _spawnedlaser
    (:Is%20Valid
      (Default|StopLaser _spawnedlaser)
      (Utilities|FlowControl|Delay 7.0)
      (Actor|DestroyActor _spawnedlaser))))

(event Custom|SpreadWingR
  (bind _spready (Timeline|SpreadWingLTimeline PlayFromStart)
    (:Update
      (Transformation|SetRelativeLocation (Variables|Default|GetRightWing) (Math|Vector|MakeVector 0.0 _spready 0.0) false false))))

(event Custom|SpreadWingL
  (bind _spready (Timeline|SpreadWingRTimeline PlayFromStart)
    (:Update
      (Transformation|SetRelativeLocation (Variables|Default|GetLeftWing) (Math|Vector|MakeVector 0.0 _spready 0.0) false false))))

(event Custom|ShootStart
  (bind _laser_charging_niagara (Variables|Default|GetLaser%20Charging%20Niagara))
  (Utilities|PlaySpreadAnimation
    (:Out
      (Components|Activation|Activate _laser_charging_niagara false)
      (Utilities|FlowControl|Sequence
        (:then_0
          (Audio|PlaySoundatLocation 0 (Transformation|GetWorldLocation (Variables|Default|GetCore)) "0, 0, 0" 1.0 1.0 0.0 0 0 0)
          (Utilities|FlowControl|Delay 3.0)
          (CallFunction|OnOffLaser)
          (CallFunction|GoBackwardParts)
          (Utilities|FlowControl|Delay 5.0)
          (CallFunction|OnOffLaser)
          (Utilities|PlayFoldAnimation))
        (:then_1
          (bind _charging (Timeline|ChargingStartTimeline PlayFromStart)
            (:Update
              (Effects|Components|ParticleSystem|SetFloatParameter _laser_charging_niagara "User.Scale" _charging))
            (:Finished
              (Components|Activation|Deactivate _laser_charging_niagara))))))))

(event Custom|RotateCore
  (bind _core (Variables|Default|GetCore))
  (bind _relativerotation (Variables|/Script/Engine.SceneComponent|GetRelativeRotation _core))
  (bind _rotationroll (Timeline|RotateCoreTimeline PlayFromStart)
    (:Update
      (Transformation|SetRelativeRotation _core (Math|Rotator|MakeRotator _rotationroll (.pitch _relativerotation) (.yaw _relativerotation)) false false))))

(event Custom|OnOffLaser
  (if (Variables|Default|GetIsShooting?)
    (Actor|Tick|SetActorTickEnabled false)
    (Variables|Default|SetIsShooting? false)
    (CallFunction|StopLaser)
    (else
      (Actor|Tick|SetActorTickEnabled true)
      (Variables|Default|SetIsShooting? true))))

(event Custom|GoBackwardParts
  (bind _gobackward (Timeline|GoBackWardPartsTimeline PlayFromStart)
    (:Update
      (Transformation|SetRelativeLocation (Variables|Default|GetCore) (Math|Vector|MakeVector _gobackward 0.0 0.0) false false))))

(event Custom|FoldWingR
  (bind _spready (Timeline|FoldWingRTimeline PlayFromStart)
    (:Update
      (Transformation|SetRelativeLocation (Variables|Default|GetRightWing) (Math|Vector|MakeVector 0.0 _spready 0.0) false false))))

(event Custom|FoldWingL
  (bind _spready (Timeline|FoldWingLTimeline PlayFromStart)
    (:Update
      (Transformation|SetRelativeLocation (Variables|Default|GetLeftWing) (Math|Vector|MakeVector 0.0 _spready 0.0) false false))))

(event EventBeginPlay
  (Utilities|Time|SetTimerbyEvent (delegate Custom|ShootStart) 12.0 true))

(event EventTick
  (params (DeltaSeconds :type Float%20%28single-precision%29))
  (CallFunction|ShootLaser))

(fn ConstructionScript)