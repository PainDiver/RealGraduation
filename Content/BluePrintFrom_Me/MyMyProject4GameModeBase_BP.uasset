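; Game mode Blueprint that shuts down an empty dedicated server session.
; On BeginPlay it starts a looping timer that periodically checks the player count in MyGameStateBase_BP's PlayerArray and prints it.
; When no players remain, it calls the MyGameInstance_BP game instance to log out the dedicated server with the current session ID and request exit.
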(event Custom|Exit
  (bind _returnvalue (Game|GetGameState))
  (bind _returnvalue_2 (Game|GetGameInstance))
  (bind _asmy_game_state_base_bp (Utilities|Casting|CastToMyGameStateBase_BP _returnvalue))
  (bind _asmy_game_instance_bp (Utilities|Casting|CastToMyGameInstance_BP _returnvalue_2))
  (bind _playerarray (Variables|/Script/Engine.GameStateBase|GetPlayerArray _asmy_game_state_base_bp))
  (bind _returnvalue_3 (Utilities|Array|Length _playerarray))
  (Utilities|IsValid _asmy_game_state_base_bp
    (:Is%20Valid
      (Development|PrintString (Utilities|String|Append (Utilities|String|MakeLiteralString "Person Check") (Utilities|String|ToString(Integer) _returnvalue_3)))
      (if (== _returnvalue_3 0)
        (Class|MyGameInstance|LogOutDediServer _asmy_game_instance_bp (Class|AdvancedSessionsLibrary|GetCurrentSessionIDasString))
        (Class|MyGameInstance|RequestExit _asmy_game_instance_bp false)))))

(event EventBeginPlay
  (|CallParentFunction)
  (Utilities|Time|SetTimerbyEvent (delegate Custom|Exit) 3e+01 true))

(event EventTick
  (params (DeltaSeconds :type Float%20%28single-precision%29)))

(fn ConstructionScript)