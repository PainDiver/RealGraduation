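; CheererDummy_BP is a crowd cheerer dummy that loops a greeting animation while turning to face the player.
; BeginPlay stops the mesh, waits a random delay to desynchronize instances, starts the animation and runs a looping timer that yaws the actor toward the player character once per second.
; The construction script gives each dummy a random color through a dynamic material instance.
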(event Custom|LookPlayer
  (bind _returnvalue (Game|GetPlayerCharacter 0))
  (Utilities|IsValid _returnvalue
    (:Is%20Valid
      (Transformation|SetActorRotation (Math|Rotator|MakeRotator 0.0 0.0 (.yaw (Math|Rotator|FindLookatRotation (Transformation|GetActorLocation) (Transformation|GetActorLocation _returnvalue))))))))

(event EventBeginPlay
  (Audio|Components|Audio|Stop (Variables|Default|GetSkeletalMesh))
  (Utilities|FlowControl|Delay (* 5 (Math|Random|RandomFloat)))
  (Components|Animation|PlayAnimation (Variables|Default|GetSkeletalMesh) "/Game/BluePrintFrom_Me/Player/CD_Chara_Anim/CD_Chara_Anim_body_Greeting.CD_Chara_Anim_body_Greeting" true)
  (Utilities|Time|SetTimerbyEvent (delegate Custom|LookPlayer) 1.0 true))

(event Collision|EventActorBeginOverlap
  (params (OtherActor :type Actor%20Object%20Reference)))

(event EventTick
  (params (DeltaSeconds :type Float%20%28single-precision%29)))

(fn ConstructionScript
  (bind _returnvalue (Rendering|Material|CreateDynamicMaterialInstance (Variables|Default|GetSkeletalMesh) 0 "/Game/BluePrintFrom_Me/Player/DynamicMaterial.DynamicMaterial" "None" :!class /Script/Engine.PrimitiveComponent))
  (Rendering|Material|SetVectorParameterValue _returnvalue "Color" (Utilities|Struct|MakeLinearColor (Math|Random|RandomFloat) (Math|Random|RandomFloat) (Math|Random|RandomFloat) 1.0) :!class /Script/Engine.MaterialInstanceDynamic))