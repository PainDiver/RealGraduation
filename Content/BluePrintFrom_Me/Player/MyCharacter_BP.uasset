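; Player character Blueprint that creates the local player's HUD and keeps the overhead name tag updated.
; On BeginPlay the locally controlled pawn adds gauge, crosshair and option widgets; the Option input toggles the menu outside ServerMap.
; A looping two-second timer polls names: the local pawn passes its GameInstance name through ServerNameSet and colors its tag green.
; Other pawns display the stored CharacterNameFromInstance once it is non-empty.
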(event Custom|nameCheck
  (bind _characternamefrominstance (Variables|Default|GetCharacterNameFromInstance))
  (if (Pawn|IsLocallyControlled)
    (bind _asmy_game_instance_bp (Utilities|Casting|CastToMyGameInstance_BP (Game|GetGameInstance)))
    (Utilities|IsValid _asmy_game_instance_bp
      (:Is%20Valid
        (CallFunction|ServerNameSet (Utilities|Text|ToText(String) (._charactername (Variables|/Script/MyProject4.MyGameInstance|Get_characterInfo _asmy_game_instance_bp))))
        (bind _asname_tag_ui (Utilities|Casting|CastToNameTag_UI (UserInterface|GetUserWidgetObject (Variables|Default|GetNameTag))))
        (Appearance|SetColorandOpacity (Variables|/Game/HUD/NameTag_UI.NameTag_UI_C|GetName _asname_tag_ui) (Utilities|Struct|MakeSlateColor "(R=0.238189,G=1.000000,B=0.000000,A=1.000000)") :!class /Script/UMG.TextBlock)
        (Rendering|Components|TextRender|SetText (Variables|/Game/HUD/NameTag_UI.NameTag_UI_C|GetName _asname_tag_ui) (Variables|Default|GetCharacterNameFromInstance))))
    (else
      (bind _asname_tag_ui_2 (Utilities|Casting|CastToNameTag_UI (UserInterface|GetUserWidgetObject (Variables|Default|GetNameTag))))
      (if (not (Utilities|Text|TextIsEmpty _characternamefrominstance))
        (bind _output_get (Variables|/Game/HUD/NameTag_UI.NameTag_UI_C|Setcharactername _asname_tag_ui_2 _characternamefrominstance))
        (Rendering|Components|TextRender|SetText (Variables|/Game/HUD/NameTag_UI.NameTag_UI_C|GetName _asname_tag_ui_2) _output_get)))))

(event Custom|ServerNameSet
  (params (NewParam :type Text))
  (Variables|Default|SetCharacterNameFromInstance NewParam))

(event EventBeginPlay
  (bind _returnvalue (Game|GetPlayerController 0))
  (Utilities|Time|SetTimerbyEvent (delegate Custom|nameCheck) 2.0 true)
  (if (Pawn|IsLocallyControlled)
    (Utilities|IsValid _returnvalue
      (:Is%20Valid
        (bind _returnvalue_2 (UserInterface|CreateWidget "/Game/HUD/Gage_UI.Gage_UI_C" _returnvalue))
        (UserInterface|Viewport|AddtoViewport _returnvalue_2 0)
        (bind _returnvalue_3 (UserInterface|CreateWidget "/Game/HUD/Crosshair_UI.Crosshair_UI_C" _returnvalue))
        (UserInterface|Viewport|AddtoViewport _returnvalue_3 0)
        (bind _returnvalue_4 (UserInterface|CreateWidget "/Game/HUD/Option_UI.Option_UI_C" _returnvalue))
        (UserInterface|Viewport|AddtoViewport _returnvalue_4 1)
        (Variables|Default|Setoption _returnvalue_4)))))

(event Collision|EventActorBeginOverlap
  (params (OtherActor :type Actor%20Object%20Reference)))

(event Input|ActionEvents|InputActionOption
  (params (Key :type Key%20Structure :default "None"))
  (bind _option (Variables|Default|Getoption))
  (:Pressed
    (bind _returnvalue (Game|GetCurrentLevelName true))
    (if (Utilities|Enum|NotEqual(Enum) _returnvalue "ServerMap")
      (Utilities|IsValid _option
        (:Is%20Valid
          (switch Utilities|FlowControl|Switch|SwitchonESlateVisibility (Widget|GetVisibility _option)
            (:Visible
              (Widget|SetVisibility _option "Hidden"))
            (:Hidden
              (Widget|SetVisibility _option "Visible"))))))))

(fn ConstructionScript)