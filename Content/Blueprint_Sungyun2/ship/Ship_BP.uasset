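; Configurable ship actor with optional spinning propellers and left and right cannon batteries that fire on their own.
; On BeginPlay, flags either unhide and animate propellers and cannons or clear their meshes (cannons only when both sides are off), swapping in a cannon hull when armed.
; Two timelines roll the propellers.
; Each cannon's looping timer, with randomised start delay and once-rolled interval, spawns BP_CannonBall at its child component's transform.
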(event EventBeginPlay
  (Variables|Default|SetLocation (Transformation|GetWorldLocation (Variables|Default|GetPivot)))
  (if (not (Variables|Bool|GetIsPropeller?))
    (Utilities|DisablePropeller
      (:Out
        _))
    (else
      (Utilities|VisiblePropeller
        (:Out
          (CallFunction|AnimatePropeller)))))
  (if (not (or (Variables|Bool|GetIsCannonL?) (Variables|Bool|GetIsCannonR?)))
    (Utilities|DisableCannonR
      (:Out
        (Utilities|DisableCannonL)))
    (else
      (Components|StaticMesh|SetStaticMesh (Variables|Default|GetBody) "/Game/Blueprint_Sungyun2/ship/Mesh/body_cannon.body_cannon")
      (if (Variables|Bool|GetIsCannonL?)
        (Utilities|VisibleCannonL
          (:Out
            (Cannon|AnimateShootCannonL))))
      (if (Variables|Bool|GetIsCannonR?)
        (Utilities|VisibleCannonR
          (:Out
            (Cannon|AnimateShootCannonR)))))))

(event Custom|PropellerSpin01
  (params (타깃 :type Scene%20Component%20Object%20Reference))
  (bind _propellerrotx (Timeline|PropellerSpinTimeline01 Play)
    (:Update
      (Transformation|SetRelativeRotation 타깃 (Math|Rotator|MakeRotator _propellerrotx 0.0 0.0) false false))))

(event Custom|PropellerSpin02
  (params (타깃 :type Scene%20Component%20Object%20Reference))
  (bind _propellerrotx (Timeline|PropellerSpinTimeline02 Play)
    (:Update
      (Transformation|SetRelativeRotation 타깃 (Math|Rotator|MakeRotator _propellerrotx 0.0 0.0) false false))))

(event Custom|ShootCannonL01
  (Game|SpawnActorfromClass "/Game/Blueprint_Sungyun2/ship/BP_CannonBall.BP_CannonBall_C" (Transformation|GetWorldTransform (Components|GetChildComponent (stale Custom|AnimateCannonL01 타깃) 0)) "Undefined" 0 0))

(event Custom|AnimateCannonL01
  (params (타깃 :type Scene%20Component%20Object%20Reference))
  (Utilities|Time|SetTimerbyEvent (delegate Custom|ShootCannonL01) (Math|Random|RandomFloatinRange (Variables|Cannon|GetMinShootInterval) (Variables|Cannon|GetMaxShootInterval)) true (Math|Random|RandomFloatinRange 0.0 1.25)))

(event Custom|AnimateCannonL02
  (params (타깃 :type Scene%20Component%20Object%20Reference))
  (Utilities|Time|SetTimerbyEvent (delegate Custom|ShootCannonL02) (Math|Random|RandomFloatinRange (Variables|Cannon|GetMinShootInterval) (Variables|Cannon|GetMaxShootInterval)) true (Math|Random|RandomFloatinRange 0.0 1.25)))

(event Custom|ShootCannonL02
  (Game|SpawnActorfromClass "/Game/Blueprint_Sungyun2/ship/BP_CannonBall.BP_CannonBall_C" (Transformation|GetWorldTransform (Components|GetChildComponent (stale Custom|AnimateCannonL02 타깃) 0)) "Undefined" 0 0))

(event Custom|AnimateCannonL08
  (params (타깃 :type Scene%20Component%20Object%20Reference))
  (Utilities|Time|SetTimerbyEvent (delegate Custom|ShootCannonL08) (Math|Random|RandomFloatinRange (Variables|Cannon|GetMinShootInterval) (Variables|Cannon|GetMaxShootInterval)) true (Math|Random|RandomFloatinRange 0.0 1.25)))

(event Custom|ShootCannonL08
  (Game|SpawnActorfromClass "/Game/Blueprint_Sungyun2/ship/BP_CannonBall.BP_CannonBall_C" (Transformation|GetWorldTransform (Components|GetChildComponent (stale Custom|AnimateCannonL08 타깃) 0)) "Undefined" 0 0))

(event Custom|AnimateCannonL07
  (params (타깃 :type Scene%20Component%20Object%20Reference))
  (Utilities|Time|SetTimerbyEvent (delegate Custom|ShootCannonL07) (Math|Random|RandomFloatinRange (Variables|Cannon|GetMinShootInterval) (Variables|Cannon|GetMaxShootInterval)) true (Math|Random|RandomFloatinRange 0.0 1.25)))

(event Custom|ShootCannonL07
  (Game|SpawnActorfromClass "/Game/Blueprint_Sungyun2/ship/BP_CannonBall.BP_CannonBall_C" (Transformation|GetWorldTransform (Components|GetChildComponent (stale Custom|AnimateCannonL07 타깃) 0)) "Undefined" 0 0))

(event Custom|AnimateCannonL06
  (params (타깃 :type Scene%20Component%20Object%20Reference))
  (Utilities|Time|SetTimerbyEvent (delegate Custom|ShootCannonL06) (Math|Random|RandomFloatinRange (Variables|Cannon|GetMinShootInterval) (Variables|Cannon|GetMaxShootInterval)) true (Math|Random|RandomFloatinRange 0.0 1.25)))

(event Custom|ShootCannonL06
  (Game|SpawnActorfromClass "/Game/Blueprint_Sungyun2/ship/BP_CannonBall.BP_CannonBall_C" (Transformation|GetWorldTransform (Components|GetChildComponent (stale Custom|AnimateCannonL06 타깃) 0)) "Undefined" 0 0))

(event Custom|AnimateCannonL04
  (params (타깃 :type Scene%20Component%20Object%20Reference))
  (Utilities|Time|SetTimerbyEvent (delegate Custom|ShootCannonL04) (Math|Random|RandomFloatinRange (Variables|Cannon|GetMinShootInterval) (Variables|Cannon|GetMaxShootInterval)) true (Math|Random|RandomFloatinRange 0.0 1.25)))

(event Custom|AnimateCannonL05
  (params (타깃 :type Scene%20Component%20Object%20Reference))
  (Utilities|Time|SetTimerbyEvent (delegate Custom|ShootCannonL05) (Math|Random|RandomFloatinRange (Variables|Cannon|GetMinShootInterval) (Variables|Cannon|GetMaxShootInterval)) true (Math|Random|RandomFloatinRange 0.0 1.25)))

(event Custom|ShootCannonL05
  (Game|SpawnActorfromClass "/Game/Blueprint_Sungyun2/ship/BP_CannonBall.BP_CannonBall_C" (Transformation|GetWorldTransform (Components|GetChildComponent (stale Custom|AnimateCannonL05 타깃) 0)) "Undefined" 0 0))

(event Custom|ShootCannonL04
  (Game|SpawnActorfromClass "/Game/Blueprint_Sungyun2/ship/BP_CannonBall.BP_CannonBall_C" (Transformation|GetWorldTransform (Components|GetChildComponent (stale Custom|AnimateCannonL04 타깃) 0)) "Undefined" 0 0))

(event Custom|AnimateCannonR08
  (params (타깃 :type Scene%20Component%20Object%20Reference))
  (Utilities|Time|SetTimerbyEvent (delegate Custom|ShootCannonR08) (Math|Random|RandomFloatinRange (Variables|Cannon|GetMinShootInterval) (Variables|Cannon|GetMaxShootInterval)) true (Math|Random|RandomFloatinRange (Variables|Default|GetMinShootDelay) (Variables|Default|GetMaxShootDelay))))

(event Custom|ShootCannonR08
  (Game|SpawnActorfromClass "/Game/Blueprint_Sungyun2/ship/BP_CannonBall.BP_CannonBall_C" (Transformation|GetWorldTransform (Components|GetChildComponent (stale Custom|AnimateCannonR08 타깃) 0)) "Undefined" 0 0))

(event Custom|AnimateCannonR07
  (params (타깃 :type Scene%20Component%20Object%20Reference))
  (Utilities|Time|SetTimerbyEvent (delegate Custom|ShootCannonR07) (Math|Random|RandomFloatinRange (Variables|Cannon|GetMinShootInterval) (Variables|Cannon|GetMaxShootInterval)) true (Math|Random|RandomFloatinRange (Variables|Default|GetMinShootDelay) (Variables|Default|GetMaxShootDelay))))

(event Custom|ShootCannonR07
  (Game|SpawnActorfromClass "/Game/Blueprint_Sungyun2/ship/BP_CannonBall.BP_CannonBall_C" (Transformation|GetWorldTransform (Components|GetChildComponent (stale Custom|AnimateCannonR07 타깃) 0)) "Undefined" 0 0))

(event Custom|AnimateCannonR06
  (params (타깃 :type Scene%20Component%20Object%20Reference))
  (Utilities|Time|SetTimerbyEvent (delegate Custom|ShootCannonR06) (Math|Random|RandomFloatinRange (Variables|Cannon|GetMinShootInterval) (Variables|Cannon|GetMaxShootInterval)) true (Math|Random|RandomFloatinRange (Variables|Default|GetMinShootDelay) (Variables|Default|GetMaxShootDelay))))

(event Custom|ShootCannonR06
  (Game|SpawnActorfromClass "/Game/Blueprint_Sungyun2/ship/BP_CannonBall.BP_CannonBall_C" (Transformation|GetWorldTransform (Components|GetChildComponent (stale Custom|AnimateCannonR06 타깃) 0)) "Undefined" 0 0))

(event Custom|AnimateCannonR05
  (params (타깃 :type Scene%20Component%20Object%20Reference))
  (Utilities|Time|SetTimerbyEvent (delegate Custom|ShootCannonR05) (Math|Random|RandomFloatinRange (Variables|Cannon|GetMinShootInterval) (Variables|Cannon|GetMaxShootInterval)) true (Math|Random|RandomFloatinRange 0.0 1.25)))

(event Custom|ShootCannonR05
  (Game|SpawnActorfromClass "/Game/Blueprint_Sungyun2/ship/BP_CannonBall.BP_CannonBall_C" (Transformation|GetWorldTransform (Components|GetChildComponent (stale Custom|AnimateCannonR05 타깃) 0)) "Undefined" 0 0))

(event Custom|AnimateCannonR04
  (params (타깃 :type Scene%20Component%20Object%20Reference))
  (Utilities|Time|SetTimerbyEvent (delegate Custom|ShootCannonR04) (Math|Random|RandomFloatinRange (Variables|Cannon|GetMinShootInterval) (Variables|Cannon|GetMaxShootInterval)) true (Math|Random|RandomFloatinRange 0.0 1.25)))

(event Custom|ShootCannonR04
  (Game|SpawnActorfromClass "/Game/Blueprint_Sungyun2/ship/BP_CannonBall.BP_CannonBall_C" (Transformation|GetWorldTransform (Components|GetChildComponent (stale Custom|AnimateCannonR04 타깃) 0)) "Undefined" 0 0))

(event Custom|AnimateCannonR03
  (params (타깃 :type Scene%20Component%20Object%20Reference))
  (Utilities|Time|SetTimerbyEvent (delegate Custom|ShootCannonR03) (Math|Random|RandomFloatinRange (Variables|Cannon|GetMinShootInterval) (Variables|Cannon|GetMaxShootInterval)) true (Math|Random|RandomFloatinRange 0.0 1.25)))

(event Custom|ShootCannonR03
  (Game|SpawnActorfromClass "/Game/Blueprint_Sungyun2/ship/BP_CannonBall.BP_CannonBall_C" (Transformation|GetWorldTransform (Components|GetChildComponent (stale Custom|AnimateCannonR03 타깃) 0)) "Undefined" 0 0))

(event Custom|AnimateCannonR02
  (params (타깃 :type Scene%20Component%20Object%20Reference))
  (Utilities|Time|SetTimerbyEvent (delegate Custom|ShootCannonR02) (Math|Random|RandomFloatinRange (Variables|Cannon|GetMinShootInterval) (Variables|Cannon|GetMaxShootInterval)) true (Math|Random|RandomFloatinRange 0.0 1.25)))

(event Custom|ShootCannonR02
  (Game|SpawnActorfromClass "/Game/Blueprint_Sungyun2/ship/BP_CannonBall.BP_CannonBall_C" (Transformation|GetWorldTransform (Components|GetChildComponent (stale Custom|AnimateCannonR02 타깃) 0)) "Undefined" 0 0))

(event Custom|AnimateCannonR01
  (params (타깃 :type Scene%20Component%20Object%20Reference))
  (Utilities|Time|SetTimerbyEvent (delegate Custom|ShootCannonR01) (Math|Random|RandomFloatinRange (Variables|Cannon|GetMinShootInterval) (Variables|Cannon|GetMaxShootInterval)) true (Math|Random|RandomFloatinRange 0.0 1.25)))

(event Custom|ShootCannonR01
  (Game|SpawnActorfromClass "/Game/Blueprint_Sungyun2/ship/BP_CannonBall.BP_CannonBall_C" (Transformation|GetWorldTransform (Components|GetChildComponent (stale Custom|AnimateCannonR01 타깃) 0)) "Undefined" 0 0))

(event Custom|AnimateCannonL03
  (params (타깃 :type Scene%20Component%20Object%20Reference))
  (Utilities|Time|SetTimerbyEvent (delegate Custom|ShootCannonL03) (Math|Random|RandomFloatinRange (Variables|Cannon|GetMinShootInterval) (Variables|Cannon|GetMaxShootInterval)) true (Math|Random|RandomFloatinRange 0.0 1.25)))

(event Custom|ShootCannonL03
  (Game|SpawnActorfromClass "/Game/Blueprint_Sungyun2/ship/BP_CannonBall.BP_CannonBall_C" (Transformation|GetWorldTransform (Components|GetChildComponent (stale Custom|AnimateCannonL03 타깃) 0)) "Undefined" 0 0))

(fn ConstructionScript)

(fn AnimatePropeller
  (Utilities|FlowControl|Sequence
    (:then_0
      (CallFunction|PropellerSpin01 (Variables|Default|GetPropeller01)))
    (:then_1
      (CallFunction|PropellerSpin02 (Variables|Default|GetPropeller02)))))

(fn AnimateShootCannonR
  (CallFunction|AnimateCannonR01 (Variables|Default|GetCannon08))
  (CallFunction|AnimateCannonR02 (Variables|Default|GetCannon07))
  (CallFunction|AnimateCannonR03 (Variables|Default|GetCannon06))
  (CallFunction|AnimateCannonR04 (Variables|Default|GetCannon05))
  (CallFunction|AnimateCannonR05 (Variables|Default|GetCannon04))
  (CallFunction|AnimateCannonR06 (Variables|Default|GetCannon03))
  (CallFunction|AnimateCannonR07 (Variables|Default|GetCannon02))
  (CallFunction|AnimateCannonR08 (Variables|Default|GetCannon01)))

(fn AnimateShootCannonL
  (CallFunction|AnimateCannonL01 (Variables|Default|GetCannon16))
  (CallFunction|AnimateCannonL02 (Variables|Default|GetCannon15))
  (CallFunction|AnimateCannonL03 (Variables|Default|GetCannon14))
  (CallFunction|AnimateCannonL04 (Variables|Default|GetCannon13))
  (CallFunction|AnimateCannonL05 (Variables|Default|GetCannon12))
  (CallFunction|AnimateCannonL06 (Variables|Default|GetCannon11))
  (CallFunction|AnimateCannonL07 (Variables|Default|GetCannon10))
  (CallFunction|AnimateCannonL08 (Variables|Default|GetCannon09)))