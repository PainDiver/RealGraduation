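; Multiplayer double-barrel turret that auto-fires at characters in range or can be ridden and fired manually.
; When unused, a detection sphere feeds random target selection; gated Delay loops turn platform yaw and body pitch toward visible targets, otherwise back to rest.
; Riding attaches the rider to the platform via server-to-multicast events, and Attack input starts timed, camera-directed fire.
; Both modes spawn paired bullets with multicast effects.
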(event OnComponentBeginOverlap(OverlapDetection)
  (params (OverlappedComponent :type Primitive%20Component%20Object%20Reference) (OtherActor :type Actor%20Object%20Reference) (OtherComp :type Primitive%20Component%20Object%20Reference) (OtherBodyIndex :type Integer) (bFromSweep :type Boolean) (SweepResult :type Hit%20Result%20Structure%20%28by%20ref%29))
  (if (not (Variables|Default|GetBeingUsed))
    ;[1 1 1] 작동 안 할 시, 형변환 객체를 바꿔주면 됨
    (bind _asmy_character_bp (Utilities|Casting|CastToMyCharacter_BP OtherActor))
    (Utilities|Array|Add (Variables|Default|GetTargetsInRange) _asmy_character_bp)
    (Utilities|IsValid (Variables|Default|GetTarget)
      (:Is%20Not%20Valid
        (CallFunction|SelectTarget)))))

(event OnComponentEndOverlap(OverlapDetection)
  (params (OverlappedComponent :type Primitive%20Component%20Object%20Reference) (OtherActor :type Actor%20Object%20Reference) (OtherComp :type Primitive%20Component%20Object%20Reference) (OtherBodyIndex :type Integer))
  (bind _targetsinrange (Variables|Default|GetTargetsInRange))
  (if (not (Variables|Default|GetBeingUsed))
    ;[1 1 1] 작동 안 할 시, 형변환 객체를 바꿔주면 됨
    (bind _asmy_character_bp (Utilities|Casting|CastToMyCharacter_BP OtherActor))
    (if (Utilities|Array|ContainsItem _targetsinrange _asmy_character_bp)
      (Utilities|Array|RemoveItem _targetsinrange _asmy_character_bp)
      (if (== _asmy_character_bp (Variables|Default|GetTarget))
        (Variables|Default|SetTarget 0)
        (CallFunction|SelectTarget)))))

(event Custom|SelectTarget
  (bind _targetsinrange (Variables|Default|GetTargetsInRange))
  (if (Utilities|Array|IsValidIndex _targetsinrange)
    (Variables|Default|SetTarget (Utilities|Array|Get(acopy) _targetsinrange (Math|Random|RandomIntegerinRange 0 (Utilities|Array|LastIndex _targetsinrange))))
    (CallFunction|BeginAimtoPlayer)
    (else
      (CallFunction|BeginResetAim))))

(event Custom|BeginAimToPlayer
  (bind _cd_turret_body (Variables|Default|GetCD_Turret_Body))
  (bind _cd_turret_platform (Variables|Default|GetCD_Turret_Platform))
  (bind _target (Variables|Default|GetTarget))
  (Utilities|FlowControl|Sequence
    (:then_0
      (goto _label Open))
    (:then_1
      (Utilities|FlowControl|Gate true :!label _label
        (:Exit
          (Utilities|IsValid _target
            (:Is%20Valid
              (Variables|Default|SetPlayerLocation (Transformation|GetActorLocation _target))
              (Variables|Default|SetIsAiming? true)
              (Transformation|SetRelativeRotation _cd_turret_platform (Math|Interpolation|RInterpTo (Variables|/Script/Engine.SceneComponent|GetRelativeRotation _cd_turret_platform) (Math|Rotator|MakeRotator 0.0 0.0 (.Yaw (Math|Rotator|BreakRotator (Math|Rotator|MakeRotfromX (Math|Transform|InverseTransformDirection (Transformation|GetActorTransform) (- (Variables|Default|GetPlayerLocation) (Transformation|GetWorldLocation (Variables|Default|GetCD_Turret_Body)))))))) (Utilities|Time|GetWorldDeltaSeconds) 1e+01) false false)
              (Transformation|SetRelativeRotation _cd_turret_body (Math|Interpolation|RInterpTo (Variables|/Script/Engine.SceneComponent|GetRelativeRotation _cd_turret_body) (Math|Rotator|MakeRotator 0.0 (.Pitch (Math|Rotator|BreakRotator (Math|Rotator|MakeRotfromX (Math|Transform|InverseTransformDirection (Transformation|GetActorTransform) (- (Variables|Default|GetPlayerLocation) (Transformation|GetWorldLocation (Variables|Default|GetCD_Turret_Body))))))) 0.0) (Utilities|Time|GetWorldDeltaSeconds) 1e+01) false false)
              (Utilities|FlowControl|Delay (Utilities|Time|GetWorldDeltaSeconds))
              (Utilities|FlowControl|Sequence
                (:then_0
                  (if (not (Variables|Default|GetBeingUsed))
                    (CallFunction|ContinueAim)))
                (:then_1
                  (Utilities|FlowControl|Delay (Variables|Default|GetShotInterval))
                  (if (not (Variables|Default|GetBeingUsed))
                    (if (Variables|Default|GetIsAiming?)
                      (CallFunction|SpawnBullet))))))
            (:Is%20Not%20Valid
              (CallFunction|CancelAim)
              (CallFunction|BeginResetAim))))))))

(event Custom|AttachActorServer
  (CallFunction|AttachActorMulti))

(event Custom|AttachActorMulti
  (bind _rider (Variables|Default|GetRider))
  (Utilities|IsValid _rider
    (:Is%20Valid
      (Transformation|AttachComponentToComponent _rider (Variables|Default|GetCD_Turret_Platform) (Variables|Default|GetSocketName) "SnapToTarget" "SnapToTarget" "KeepWorld" false))))

(event Custom|MultiEffect
  (params (Location :type Vector))
  (Effects|SpawnEmitteratLocation "/Game/Blueprint_Sungyun2/StarterContent/Particles/P_Explosion.P_Explosion" Location)
  (Audio|Components|Audio|Play (Variables|Default|GetAudio) 0.0)
  (Components|Timeline|PlayfromStart (Variables|Default|GetCD_DoubleTurret_Recoil)))

(event Custom|CancelAim
  (bind _cd_turret_body (Variables|Default|GetCD_Turret_Body))
  (bind _cd_turret_platform (Variables|Default|GetCD_Turret_Platform))
  (bind _target (Variables|Default|GetTarget))
  (Utilities|FlowControl|Gate true) ; enters at Close
)

(event Custom|ContinueAim
  (bind _cd_turret_body (Variables|Default|GetCD_Turret_Body))
  (bind _cd_turret_platform (Variables|Default|GetCD_Turret_Platform))
  (bind _target (Variables|Default|GetTarget))
  (Utilities|IsValid (Variables|Default|GetTarget)
    (:Is%20Valid
      (bind _isblocking_ (CallFunction|TracePlayer))
      (if _isblocking_
        (CallFunction|CancelAim :!label _label)
        (CallFunction|BeginResetAim)
        (else
          (Utilities|FlowControl|Gate true
            (:Exit
              (Utilities|IsValid _target
                (:Is%20Valid
                  (Variables|Default|SetPlayerLocation (Transformation|GetActorLocation _target))
                  (Variables|Default|SetIsAiming? true)
                  (Transformation|SetRelativeRotation _cd_turret_platform (Math|Interpolation|RInterpTo (Variables|/Script/Engine.SceneComponent|GetRelativeRotation _cd_turret_platform) (Math|Rotator|MakeRotator 0.0 0.0 (.Yaw (Math|Rotator|BreakRotator (Math|Rotator|MakeRotfromX (Math|Transform|InverseTransformDirection (Transformation|GetActorTransform) (- (Variables|Default|GetPlayerLocation) (Transformation|GetWorldLocation (Variables|Default|GetCD_Turret_Body)))))))) (Utilities|Time|GetWorldDeltaSeconds) 1e+01) false false)
                  (Transformation|SetRelativeRotation _cd_turret_body (Math|Interpolation|RInterpTo (Variables|/Script/Engine.SceneComponent|GetRelativeRotation _cd_turret_body) (Math|Rotator|MakeRotator 0.0 (.Pitch (Math|Rotator|BreakRotator (Math|Rotator|MakeRotfromX (Math|Transform|InverseTransformDirection (Transformation|GetActorTransform) (- (Variables|Default|GetPlayerLocation) (Transformation|GetWorldLocation (Variables|Default|GetCD_Turret_Body))))))) 0.0) (Utilities|Time|GetWorldDeltaSeconds) 1e+01) false false)
                  (Utilities|FlowControl|Delay (Utilities|Time|GetWorldDeltaSeconds))
                  (Utilities|FlowControl|Sequence
                    (:then_0
                      (if (not (Variables|Default|GetBeingUsed))
                        (CallFunction|ContinueAim)))
                    (:then_1
                      (Utilities|FlowControl|Delay (Variables|Default|GetShotInterval))
                      (if (not (Variables|Default|GetBeingUsed))
                        (if (Variables|Default|GetIsAiming?)
                          (CallFunction|SpawnBullet))))))
                (:Is%20Not%20Valid
                  (goto _label))))))))
    (:Is%20Not%20Valid
      (goto _label))))

(event Custom|BeginResetAim
  (bind _returnvalue (Math|Rotator|MakeRotator 0.0 0.0 0.0))
  (bind _returnvalue_2 (Math|Rotator|MakeRotator 0.0 0.0 0.0))
  (bind _returnvalue_3 (Utilities|Time|GetWorldDeltaSeconds))
  (bind _returnvalue_4 (Utilities|Time|GetWorldDeltaSeconds))
  (bind _cd_turret_body (Variables|Default|GetCD_Turret_Body))
  (bind _cd_turret_platform (Variables|Default|GetCD_Turret_Platform))
  (bind _relativerotation (Variables|/Script/Engine.SceneComponent|GetRelativeRotation _cd_turret_platform))
  (bind _relativerotation_2 (Variables|/Script/Engine.SceneComponent|GetRelativeRotation _cd_turret_body))
  (bind _returnvalue_5 (Math|Interpolation|RInterpTo _relativerotation_2 _returnvalue _returnvalue_4 25.0))
  (bind _returnvalue_6 (Math|Interpolation|RInterpTo _relativerotation _returnvalue_2 _returnvalue_3 25.0))
  (Utilities|FlowControl|Sequence
    (:then_0
      (goto _label Open))
    (:then_1
      (Utilities|FlowControl|Gate true :!label _label
        (:Exit
          (Utilities|IsValid (Variables|Default|GetTarget)
            (:Is%20Valid
              (CallFunction|CancelReset :!label _label_2))
            (:Is%20Not%20Valid
              (if (and (Math|Rotator|Equal(Rotator) _returnvalue_6 "0, 0, 0" 0.01) (Math|Rotator|Equal(Rotator) _returnvalue_5 "0, 0, 0" 0.01))
                (goto _label_2)
                (else
                  (Variables|Default|SetIsAiming? false)
                  (Transformation|SetRelativeRotation (Variables|Default|GetCD_Turret_Platform) _returnvalue_6 false false)
                  (Transformation|SetRelativeRotation (Variables|Default|GetCD_Turret_Body) _returnvalue_5 false false)
                  (Utilities|FlowControl|Delay (Utilities|Time|GetWorldDeltaSeconds))
                  (CallFunction|ContinueReset))))))))))

(event Custom|CancelReset
  (bind _returnvalue (Math|Rotator|MakeRotator 0.0 0.0 0.0))
  (bind _returnvalue_2 (Math|Rotator|MakeRotator 0.0 0.0 0.0))
  (bind _returnvalue_3 (Utilities|Time|GetWorldDeltaSeconds))
  (bind _returnvalue_4 (Utilities|Time|GetWorldDeltaSeconds))
  (bind _cd_turret_body (Variables|Default|GetCD_Turret_Body))
  (bind _cd_turret_platform (Variables|Default|GetCD_Turret_Platform))
  (bind _relativerotation (Variables|/Script/Engine.SceneComponent|GetRelativeRotation _cd_turret_platform))
  (bind _relativerotation_2 (Variables|/Script/Engine.SceneComponent|GetRelativeRotation _cd_turret_body))
  (bind _returnvalue_5 (Math|Interpolation|RInterpTo _relativerotation_2 _returnvalue _returnvalue_4 25.0))
  (bind _returnvalue_6 (Math|Interpolation|RInterpTo _relativerotation _returnvalue_2 _returnvalue_3 25.0))
  (Utilities|FlowControl|Gate true) ; enters at Close
)

(event Custom|ContinueReset
  (bind _returnvalue (Math|Rotator|MakeRotator 0.0 0.0 0.0))
  (bind _returnvalue_2 (Math|Rotator|MakeRotator 0.0 0.0 0.0))
  (bind _returnvalue_3 (Utilities|Time|GetWorldDeltaSeconds))
  (bind _returnvalue_4 (Utilities|Time|GetWorldDeltaSeconds))
  (bind _cd_turret_body (Variables|Default|GetCD_Turret_Body))
  (bind _cd_turret_platform (Variables|Default|GetCD_Turret_Platform))
  (bind _relativerotation (Variables|/Script/Engine.SceneComponent|GetRelativeRotation _cd_turret_platform))
  (bind _relativerotation_2 (Variables|/Script/Engine.SceneComponent|GetRelativeRotation _cd_turret_body))
  (bind _returnvalue_5 (Math|Interpolation|RInterpTo _relativerotation_2 _returnvalue _returnvalue_4 25.0))
  (bind _returnvalue_6 (Math|Interpolation|RInterpTo _relativerotation _returnvalue_2 _returnvalue_3 25.0))
  (Utilities|FlowControl|Gate true
    (:Exit
      (Utilities|IsValid (Variables|Default|GetTarget)
        (:Is%20Valid
          (CallFunction|CancelReset :!label _label))
        (:Is%20Not%20Valid
          (if (and (Math|Rotator|Equal(Rotator) _returnvalue_6 "0, 0, 0" 0.01) (Math|Rotator|Equal(Rotator) _returnvalue_5 "0, 0, 0" 0.01))
            (goto _label)
            (else
              (Variables|Default|SetIsAiming? false)
              (Transformation|SetRelativeRotation (Variables|Default|GetCD_Turret_Platform) _returnvalue_6 false false)
              (Transformation|SetRelativeRotation (Variables|Default|GetCD_Turret_Body) _returnvalue_5 false false)
              (Utilities|FlowControl|Delay (Utilities|Time|GetWorldDeltaSeconds))
              (CallFunction|ContinueReset))))))))

(event Custom|SpawnBulletServerInPossess
  (bind _bullet_spawner_l (Variables|Default|GetBullet_Spawner_L))
  (bind _bullet_spawner_r (Variables|Default|GetBullet_Spawner_R))
  (bind _returnvalue (Transformation|GetWorldTransform _bullet_spawner_r))
  (bind _returnvalue_2 (Transformation|GetWorldTransform _bullet_spawner_l))
  (Utilities|FlowControl|Sequence
    (:then_0
      (bind _returnvalue_3 (Game|SpawnActorfromClass "/Game/Blueprint_Sungyun2/BluePrints/Objects/CD_Projectile/CD_Bullet_BP.CD_Bullet_BP_C" (Math|Transform|MakeTransform (.location _returnvalue_2) (.rotation _returnvalue_2) "1,1,1") "Undefined" 0 0))
      (Variables|/Script/Engine.MovementComponent|SetVelocity (Variables|/Game/Blueprint_Sungyun2/BluePrints/Objects/CD_Projectile/CD_Bullet_BP.CD_Bullet_BP_C|GetProjectileMovement _returnvalue_3) (+ (* (Math|Vector|GetForwardVector (Variables|Default|GetCamera)) (Variables|/Script/Engine.ProjectileMovementComponent|GetInitialSpeed (Variables|/Game/Blueprint_Sungyun2/BluePrints/Objects/CD_Projectile/CD_Bullet_BP.CD_Bullet_BP_C|GetProjectileMovement _returnvalue_3))) (Math|Vector|MakeVector 0.0 0.0 (- (.z (Transformation|GetWorldLocation (Variables|Default|GetCamera))) (.z (Transformation|GetWorldLocation (Variables|Default|GetBullet_Spawner_L)))))))
      (CallFunction|MultiEffect (.location _returnvalue_2)))
    (:then_1
      (bind _returnvalue_4 (Game|SpawnActorfromClass "/Game/Blueprint_Sungyun2/BluePrints/Objects/CD_Projectile/CD_Bullet_BP.CD_Bullet_BP_C" (Math|Transform|MakeTransform (.location _returnvalue) (.rotation _returnvalue) "1,1,1") "Undefined" 0 0))
      (Variables|/Script/Engine.MovementComponent|SetVelocity (Variables|/Game/Blueprint_Sungyun2/BluePrints/Objects/CD_Projectile/CD_Bullet_BP.CD_Bullet_BP_C|GetProjectileMovement _returnvalue_4) (+ (* (Math|Vector|GetForwardVector (Variables|Default|GetCamera)) (Variables|/Script/Engine.ProjectileMovementComponent|GetInitialSpeed (Variables|/Game/Blueprint_Sungyun2/BluePrints/Objects/CD_Projectile/CD_Bullet_BP.CD_Bullet_BP_C|GetProjectileMovement _returnvalue_4))) (Math|Vector|MakeVector 0.0 0.0 (- (.z (Transformation|GetWorldLocation (Variables|Default|GetCamera))) (.z (Transformation|GetWorldLocation (Variables|Default|GetBullet_Spawner_R)))))))
      (CallFunction|MultiEffect (.location _returnvalue)))))

(event Custom|SpawnBullet
  (bind _bullet_spawner_l (Variables|Default|GetBullet_Spawner_L))
  (bind _bullet_spawner_r (Variables|Default|GetBullet_Spawner_R))
  (bind _returnvalue (Transformation|GetWorldTransform _bullet_spawner_l))
  (bind _returnvalue_2 (Transformation|GetWorldTransform _bullet_spawner_r))
  (Utilities|FlowControl|Sequence
    (:then_0
      (Game|SpawnActorfromClass "/Game/Blueprint_Sungyun2/BluePrints/Objects/CD_Projectile/CD_Bullet_BP.CD_Bullet_BP_C" (Math|Transform|MakeTransform (.location _returnvalue) (.rotation _returnvalue) "1,1,1") "Undefined" 0 0)
      (CallFunction|MultiEffect (.location _returnvalue)))
    (:then_1
      (Game|SpawnActorfromClass "/Game/Blueprint_Sungyun2/BluePrints/Objects/CD_Projectile/CD_Bullet_BP.CD_Bullet_BP_C" (Math|Transform|MakeTransform (.location _returnvalue_2) (.rotation _returnvalue_2) "1,1,1") "Undefined" 0 0)
      (CallFunction|MultiEffect (.location _returnvalue_2)))))

(event EventBeginPlay
  (Components|Sphere|SetSphereRadius (Variables|Default|GetOverlapDetection) (Variables|Default|GetSensingRange) true)
  (|CallParentFunction))

(event EventPossessed
  (params (NewController :type Controller%20Object%20Reference))
  (Utilities|FlowControl|Sequence
    (:then_0
      (Transformation|SetRelativeRotation (Variables|Default|GetCD_Turret_Platform) "0, 0, 0" false false))
    (:then_1
      (Transformation|SetRelativeRotation (Variables|Default|GetCD_Turret_Body) "0, 0, 0" false false))))

(event EventRide
  (params (DelegateCaller :type Actor%20Object%20Reference))
  (|CallParentFunction DelegateCaller)
  (CallFunction|AttachActorServer))

(event Input|ActionEvents|InputActionAttack
  (params (Key :type Key%20Structure))
  (:Pressed
    (if (not (Variables|Default|GetIsShooting))
      (Variables|Default|SetIsShooting true)
      (CallFunction|SpawnBulletServerinPossess)
      (bind _returnvalue (Utilities|Time|SetTimerbyEvent (delegate Custom|SpawnBulletServerInPossess) (Variables|Default|GetShotInterval) true))
      (Variables|Default|SetTimerHandle _returnvalue)))
  (:Released
    (Utilities|Time|ClearandInvalidateTimerbyHandle (Variables|Default|GetTimerHandle))
    (Utilities|FlowControl|Delay (Variables|Default|GetShotInterval))
    (Variables|Default|SetIsShooting false)))

(fn ConstructionScript)

(fn TracePlayer
  (bind _target (Variables|Default|GetTarget))
  (bind _returnvalue (Collision|LineTraceByChannel (Transformation|GetWorldLocation (Variables|Default|GetCD_Turret_Body)) (Transformation|GetActorLocation _target) "TraceTypeQuery1" false (Utilities|Array|MakeArray self _target) "None"))
  (return _returnvalue))