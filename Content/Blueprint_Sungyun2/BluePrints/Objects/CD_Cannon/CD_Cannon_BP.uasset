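; A rideable cannon that spawns bombs at its spawner component, firing automatically on a timer while not in use and on Attack input.
; BeginPlay sets the barrel pitch and starts the looping timer, whose shots run only on authority.
; Ride calls the parent, then snaps the rider to the cannon through a server-to-multicast event chain.
; Held Attack repeats ShootBomb without an authority check, with a cooldown after release.
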(event Custom|ShootBomb
  (Game|SpawnActorfromClass (Variables|Default|GetSpawnedActor) (Transformation|GetWorldTransform (Variables|Default|GetCD_Bomb_Spawner)) "Undefined" 0 0))

(event Custom|AttachActorServer
  (CallFunction|AttachActorMulti))

(event Custom|AttachActorMulti
  (bind _rider (Variables|Default|GetRider))
  (Utilities|IsValid _rider
    (:Is%20Valid
      (Transformation|AttachComponentToComponent _rider (Variables|Default|GetCube) (Variables|Default|GetSocketName) "SnapToTarget" "SnapToTarget" "KeepWorld" true))))

(event Custom|Shoot
  (Networking|SwitchHasAuthority
    (:Authority
      (if (not (Variables|Default|GetBeingUsed))
        (CallFunction|ShootBomb)))))

(event EventBeginPlay
  (bind _cd_cannon_barrel (Variables|Default|GetCD_Cannon_Barrel))
  (bind _returnvalue (Transformation|GetWorldRotation _cd_cannon_barrel))
  (Utilities|Time|SetTimerbyEvent (delegate Custom|Shoot) (Variables|Default|GetShotInterval) true)
  (Transformation|SetWorldRotation _cd_cannon_barrel (Math|Rotator|MakeRotator (.roll _returnvalue) (Variables|Default|GetShotDegree) (.yaw _returnvalue)) false false)
  (|CallParentFunction))

(event Collision|EventActorBeginOverlap
  (params (OtherActor :type Actor%20Object%20Reference)))

(event EventRide
  (params (DelegateCaller :type Actor%20Object%20Reference))
  (|CallParentFunction DelegateCaller)
  (CallFunction|AttachActorServer))

(event Input|ActionEvents|InputActionAttack
  (params (Key :type Key%20Structure :default "None"))
  (:Pressed
    (if (not (Variables|Default|GetIsShooting))
      (Variables|Default|SetIsShooting true)
      (CallFunction|ShootBomb)
      (bind _returnvalue (Utilities|Time|SetTimerbyEvent (delegate Custom|ShootBomb) (Variables|Default|GetShotInterval) true))
      (Variables|Default|SetTimerHandle _returnvalue)))
  (:Released
    (Utilities|Time|ClearandInvalidateTimerbyHandle (Variables|Default|GetTimerHandle))
    (Utilities|FlowControl|Delay (Variables|Default|GetShotInterval))
    (Variables|Default|SetIsShooting false)))

(fn ConstructionScript)