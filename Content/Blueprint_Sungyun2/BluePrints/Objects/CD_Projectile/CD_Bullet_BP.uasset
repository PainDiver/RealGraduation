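; CD_Bullet_BP is a projectile with a ProjectileMovement component that knocks back the player character on overlap.
; It takes the normalized bullet-to-character direction, flattens and scales it, adds a small upward lift, and applies a mass-independent velocity-change impulse.
; Flattening follows normalization, so vertical offset weakens the horizontal push.
; The bullet destroys itself after hitting a MyCharacter_BP; other overlaps, stops and bounces do nothing.
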(event OnProjectileStop(ProjectileMovement)
  (params (ImpactResult :type Hit%20Result%20Structure%20%28by%20ref%29)))

(event OnProjectileBounce(ProjectileMovement)
  (params (ImpactResult :type Hit%20Result%20Structure%20%28by%20ref%29) (ImpactVelocity :type Vector%20%28by%20ref%29 :default "0, 0, 0")))

(event EventBeginPlay)

(event EventTick
  (params (DeltaSeconds :type Float%20%28single-precision%29)))

(event Collision|EventActorBeginOverlap
  (params (OtherActor :type Actor%20Object%20Reference))
  (bind _returnvalue (Transformation|GetActorLocation OtherActor))
  (bind _returnvalue_2 (Transformation|GetActorLocation))
  (bind _returnvalue_3 (- _returnvalue _returnvalue_2))
  (bind _returnvalue_4 (Math|Vector|Normalize _returnvalue_3))
  (bind (_x _y) (Math|Vector|BreakVector _returnvalue_4))
  (bind _returnvalue_5 (Math|Vector|MakeVector _x _y 0.0))
  (bind _returnvalue_6 (* _returnvalue_5 2000))
  (bind (_x_2 _y_2) (Math|Vector|BreakVector _returnvalue_6))
  (bind _asmy_character_bp (Utilities|Casting|CastToMyCharacter_BP OtherActor))
  (Physics|AddImpulse (Variables|/Script/Engine.Character|GetCharacterMovement _asmy_character_bp) (Math|Vector|MakeVector _x_2 _y_2 5e+01) true)
  (Actor|DestroyActor))

(fn ConstructionScript)