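; Bomb projectile that explodes once it slows below a minimum velocity or its remaining lifespan runs low.
; A throttled Tick, set to a half-second interval, checks these conditions only on the authority.
; Detonation fires a radial force impulse, calls ExplosionInServer, which passes the particle template to ExplosionInClient to spawn a scaled-up explosion emitter, then destroys the actor.
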(event Custom|ExplosionInServer
  (CallFunction|ExplosioninClient "/Game/StarterContent/Particles/P_Explosion.P_Explosion"))

(event Custom|ExplosionInClient
  (params (EmitterTemplate :type Particle%20System%20Object%20Reference))
  (Effects|SpawnEmitteratLocation EmitterTemplate (Transformation|GetActorLocation) "0, 0, 0" "6.000000,6.000000,6.000000"))

(event Custom|BlowUp
  (if (or (< (Actor|GetLifeSpan) 3.1) (< (Math|Vector|VectorLength (Transformation|GetVelocity)) (Variables|Default|GetMinVelocity)))
    (Class|RadialForceComponent|FireImpulse (Variables|Default|GetRadialForce))
    (CallFunction|ExplosioninServer)
    (Actor|DestroyActor)))

(event EventBeginPlay
  (Actor|Tick|SetActorTickInterval 0.5))

(event Collision|EventActorBeginOverlap
  (params (OtherActor :type Actor%20Object%20Reference)))

(event EventTick
  (params (DeltaSeconds :type Float%20%28single-precision%29))
  (Networking|SwitchHasAuthority
    (:Authority
      (CallFunction|Blowup))))

(fn ConstructionScript)