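; Player character for a networked game, with swimming, ziplines, spline portal jumps, generic interaction and a name tag.
; Input branches on authority, sending remote calls through Server events into shared Client or Multicast events.
; Ziplines and portals drive the capsule with MoveComponentTo while switching movement modes, guarded by DoOnce.
; The local player sends its GameInstance name to the server; other copies poll until it arrives, then fill the tag.
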(event Custom|Server%20Interact
  ;[1 1 1] Set Interaction
  (CallFunction|MulticastInteract))

(event Custom|Multicast%20Interact
  ;[1 1 1] Set Interaction
  (Class|BPIInteractableObject|StartInteraction(Message) (Variables|Default|Getinteractable%20actor) self))

(event Custom|ServerNameSet
  (params (NewParam :type Text))
  (Variables|Default|SetCharacterNameFromInstance NewParam))

(event Custom|Client%20Zipline
  (bind _zip_start_postion (Variables|Default|GetZip%20Start%20Postion))
  (bind _zip_end_postion (Variables|Default|GetZip%20End%20Postion))
  (bind _returnvalue (+ _zip_end_postion "0, 0,-90.000000"))
  ;[1 1 1] ZipLine
  (Utilities|FlowControl|DoOnce false :!label _label
    (:Completed
      (if (Variables|Default|GetZip%20Enable)
        (Pawn|Components|CharacterMovement|SetMovementMode (Variables|Character|GetCharacterMovement) "MOVE_Flying" 0)
        (Components|MoveComponentTo (Variables|Default|GetCapsuleComponent) (+ _zip_start_postion "0, 0,-90.000000") (Math|Rotator|MakeRotator 0.0 0.0 (.yaw (Math|Rotator|FindLookatRotation _zip_start_postion (Variables|Default|GetZip%20End%20Postion)))) false true 0.1 false)
        (Animation|PlayAnimMontage 0 1.0 "None")
        (Components|MoveComponentTo (Variables|Default|GetCapsuleComponent) _returnvalue (Transformation|GetActorRotation) false true (/ (Math|Vector|Distance(Vector) _returnvalue (Variables|Default|GetZip%20Start%20Postion)) 1e+03) false)
        (Animation|StopAnimMontage "/Game/BluePrintFrom_ChanHyeok/Zipline/CD_Chara_Hanging_Montage.CD_Chara_Hanging_Montage")
        (Pawn|Components|CharacterMovement|SetMovementMode (Variables|Character|GetCharacterMovement) "MOVE_Falling" 0)
        (goto _label Reset)
        (else
          (goto _label Reset))))))

(event Custom|Server%20Zipline
  ;[1 1 1] ZipLine
  (CallFunction|ClientZipline))

(event Custom|Client%20Swimming
  (params (InputPin :type Float%20%28single-precision%29))
  ;[1 1 1] Swimming
  (if (Utilities|Enum|Equal(Enum) (Variables|/Script/Engine.CharacterMovementComponent|GetMovementMode (Variables|Character|GetCharacterMovement)) "MOVE_Swimming")
    (Animation|PlayAnimMontage 0 1.0 "None")
    (Pawn|Input|AddMovementInput (Math|Vector|GetForwardVector (Transformation|GetWorldRotation (Variables|Default|Get_camera))) InputPin false)
    (else
      (Pawn|Input|AddMovementInput (Math|Vector|GetForwardVector (Pawn|GetControlRotation :!class /Script/Engine.Pawn)) InputPin false))))

(event Custom|Server%20Swim%20Jump
  ;[1 1 1] Swimming
  (CallFunction|ClientSwimJump))

(event Custom|Client%20Swim%20Jump
  ;[1 1 1] Swimming
  (if (Utilities|Enum|Equal(Enum) (Variables|/Script/Engine.CharacterMovementComponent|GetMovementMode (Variables|Character|GetCharacterMovement)) "MOVE_Swimming")
    (Character|LaunchCharacter "0.000000, 0,900.000000" false true)
    (Pawn|Components|CharacterMovement|SetMovementMode (Variables|Character|GetCharacterMovement) "MOVE_Walking" 0)
    (Pawn|Components|CharacterMovement|SetMovementMode (Variables|Character|GetCharacterMovement) "MOVE_Swimming" 0)
    (else
      (Character|Jump))))

(event Custom|Server%20Swimming
  (params (InputPin :type Float%20%28single-precision%29))
  ;[1 1 1] Swimming
  (CallFunction|ClientSwimming InputPin))

(event EventBeginPlay
  (bind _characternamefrominstance (Variables|Default|GetCharacterNameFromInstance))
  (if (Pawn|IsLocallyControlled self)
    (Utilities|FlowControl|Delay 2.0)
    (bind _asmy_game_instance_bp (Utilities|Casting|CastToMyGameInstance_BP (Game|GetGameInstance)))
    (CallFunction|ServerNameSet (Utilities|Text|ToText(String) (._CharacterName (Utilities|Struct|BreakCharacterInfo (Variables|/Script/MyProject4.MyGameInstance|Get_characterInfo _asmy_game_instance_bp)))))
    (else
      (Utilities|FlowControl|Delay 0.5 :!label _label)
      (bind _asname_tag_ui (Utilities|Casting|CastToNameTag_UI (UserInterface|GetUserWidgetObject (Variables|Default|GetNameTag self))))
      (if (Utilities|Text|TextIsEmpty _characternamefrominstance)
        (goto _label)
        (else
          (Variables|/Game/HUD/NameTag_UI.NameTag_UI_C|Setcharactername _asname_tag_ui _characternamefrominstance))))))

(event Collision|EventActorBeginOverlap
  (params (OtherActor :type Actor%20Object%20Reference)))

(event EventStartPortalJump
  (params (portal_spline :type Spline%20Component%20Object%20Reference) (directionNewParam :type Integer))
  (bind _capsulecomponent (Variables|Default|GetCapsuleComponent))
  ;[1 1 1] Portal Loop
  (Utilities|FlowControl|DoOnce false :!label _label
    (:Completed
      (Variables|portaljump|SetPortal%20Spline portal_spline)
      (Pawn|Components|CharacterMovement|SetMovementMode (Variables|Character|GetCharacterMovement) "MOVE_None" 0)
      (bind _output_get (Variables|PortalJump|Setportal_distance 0.0))
      (if (< _output_get (Spline|GetSplineLength (Variables|portaljump|GetPortal%20Spline))) :!label _label_2
        (Components|MoveComponentTo _capsulecomponent (.location (Spline|GetTransformatDistanceAlongSpline (Variables|portaljump|GetPortal%20Spline) (Variables|PortalJump|Getportal_distance) "World" false)) (.rotation (Spline|GetTransformatDistanceAlongSpline (Variables|portaljump|GetPortal%20Spline) (Variables|PortalJump|Getportal_distance) "World" false)) false false 0.2 false)
        (Variables|PortalJump|Setportal_distance (+ (Variables|PortalJump|Getportal_distance) 3e+02))
        (goto _label_2)
        (else
          (Variables|PortalJump|Setportal_distance (Spline|GetSplineLength (Variables|portaljump|GetPortal%20Spline)))
          (Components|MoveComponentTo _capsulecomponent (.location (Spline|GetTransformatDistanceAlongSpline (Variables|portaljump|GetPortal%20Spline) (Variables|PortalJump|Getportal_distance) "World" false)) (.rotation (Spline|GetTransformatDistanceAlongSpline (Variables|portaljump|GetPortal%20Spline) (Variables|PortalJump|Getportal_distance) "World" false)) false false 0.2 false)
          (Pawn|Components|CharacterMovement|SetMovementMode (Variables|Character|GetCharacterMovement) "MOVE_Walking" 0)
          (Character|LaunchCharacter (* (Transformation|GetActorForwardVector) 8e+02) false false)
          (goto _label Reset))))))

(event EventSetZipline
  (params (enable :type Boolean) (start%20postion :type Vector :default "0, 0, 0") (end%20postion :type Vector :default "0, 0, 0"))
  ;[1 1 1] ZipLine
  (Variables|Default|SetZip%20Enable enable)
  (Variables|Default|SetZip%20Start%20Postion start%20postion)
  (Variables|Default|SetZip%20End%20Postion end%20postion))

(event EventSetInteractable
  (params (interactable :type Actor%20Object%20Reference))
  ;[1 1 1] Set Interaction
  (Variables|Default|Setinteractable%20actor interactable))

(event Input|ActionEvents|InputActionInteract
  (params (Key :type Key%20Structure :default "None"))
  ;[1 1 1] ZipLine
  (:Pressed
    (Networking|SwitchHasAuthority
      (:Authority
        (CallFunction|ClientZipline))
      (:Remote
        (CallFunction|ServerZipline)))))

(event Input|ActionEvents|InputActionInteract
  (params (Key :type Key%20Structure :default "None"))
  ;[1 1 1] Set Interaction
  (:Pressed
    (Utilities|IsValid (Variables|Default|Getinteractable%20actor)
      (:Is%20Valid
        (Networking|SwitchHasAuthority
          (:Authority
            (CallFunction|MulticastInteract))
          (:Remote
            (CallFunction|ServerInteract)))))))

(event Input|AxisEvents|InputAxisMoveForward
  (params (AxisValue :type Float%20%28single-precision%29))
  ;[1 1 1] Swimming
  (Networking|SwitchHasAuthority
    (:Authority
      (CallFunction|ClientSwimming AxisValue))
    (:Remote
      (CallFunction|ServerSwimming AxisValue))))

(event Input|KeyboardEvents|SpaceBar
  (params (Key :type Key%20Structure :default "None"))
  ;[1 1 1] Swimming
  (:Pressed
    (Networking|SwitchHasAuthority
      (:Authority
        (CallFunction|ClientSwimJump))
      (:Remote
        (CallFunction|ServerSwimJump)))))

(fn ConstructionScript)

(fn GetClientController
  (return (Pawn|GetController self)))