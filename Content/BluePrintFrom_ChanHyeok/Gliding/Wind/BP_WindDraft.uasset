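; BP_WindDraft is an updraft volume that boosts the player upward while gliding.
; When MyCharacter_BP begins or ends overlap with its Box, it checks the ParkourComponent gliding flag and calls LaunchCharacter with a fixed upward velocity.
; The impulse fires once on entry and once on exit, adding to existing velocity, with no continuous lift inside the box.
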(event OnComponentBeginOverlap(Box)
  (params (OverlappedComponent :type Primitive%20Component%20Object%20Reference) (OtherActor :type Actor%20Object%20Reference) (OtherComp :type Primitive%20Component%20Object%20Reference) (OtherBodyIndex :type Integer) (bFromSweep :type Boolean) (SweepResult :type Hit%20Result%20Structure%20%28by%20ref%29))
  (bind _asmy_character_bp (Utilities|Casting|CastToMyCharacter_BP OtherActor))
  (Utilities|IsValid _asmy_character_bp
    (:Is%20Valid
      (if (Variables|/Script/MyProject4.MyCharacterParkourComponent|Get_bIsGliding (Variables|/Script/MyProject4.MyCharacter|Get_parkourComponent _asmy_character_bp))
        (Character|LaunchCharacter _asmy_character_bp "0, 0,500.000000" false false)))))

(event OnComponentEndOverlap(Box)
  (params (OverlappedComponent :type Primitive%20Component%20Object%20Reference) (OtherActor :type Actor%20Object%20Reference) (OtherComp :type Primitive%20Component%20Object%20Reference) (OtherBodyIndex :type Integer))
  (bind _asmy_character_bp (Utilities|Casting|CastToMyCharacter_BP OtherActor))
  (Utilities|IsValid _asmy_character_bp
    (:Is%20Valid
      (if (Variables|/Script/MyProject4.MyCharacterParkourComponent|Get_bIsGliding (Variables|/Script/MyProject4.MyCharacter|Get_parkourComponent _asmy_character_bp))
        (Character|LaunchCharacter _asmy_character_bp "0, 0,500.000000" false false)))))

(event EventBeginPlay)

(event Collision|EventActorBeginOverlap
  (params (OtherActor :type Actor%20Object%20Reference)))

(event EventTick
  (params (DeltaSeconds :type Float%20%28single-precision%29)))

(fn ConstructionScript)