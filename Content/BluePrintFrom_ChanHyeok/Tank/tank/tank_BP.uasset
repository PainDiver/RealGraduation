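; Tank Blueprint that animates left and right caterpillar tracks using RailPiece mesh instances placed along the LCaterpillar and RCaterpillar splines.
; BeginPlay spaces the instances evenly at constant velocity, with hard-coded index offsets separating the right track from the left.
; Per-side forward and backward events shift instances in tenth-of-a-link steps via wrapping counters, looping the end piece.
; Each pass dirties render state only on its last instance.
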(event Custom|RCaterBackward
  (bind _lastindex (Variables|Default|GetLastIndex))
  (bind _returnvalue (* _lastindex 2))
  (for _index (range 26 _returnvalue)
    (Components|InstancedStaticMesh|UpdateInstanceTransform (Variables|Default|GetRailPiece) (- _index 1) (Spline|GetTransformatTime (Variables|Default|GetRCaterpillar) (* (+ (Math|Conversions|ToFloat(Integer) (- (Math|Integer|SelectInt 50 _index (== _index _returnvalue)) 25)) (* -1 (Utilities|Select :Index (Variables|Default|GetRSelectIntegar) :Option%200 0.0 :Option%201 0.1 :Option%202 0.2 :Option%203 0.3 :Option%204 0.4 :Option%205 0.5 :Option%206 0.6 :Option%207 0.7 :Option%208 0.8 :Option%209 0.9))) (/ 1.0 (Math|Conversions|ToFloat(Integer) _lastindex))) "World" true false) true (== _index _returnvalue) false))
  (bind _result (Math|Integer|IncrementInt (Variables|Default|GetRSelectIntegar))
    (:%20%20
      (if (== _result 10)
        (Variables|Default|SetRSelectIntegar 0)))))

(event Custom|RCaterForward
  (bind _lastindex (Variables|Default|GetLastIndex))
  (bind _returnvalue (* _lastindex 2))
  (for _index (range 26 _returnvalue)
    (Components|InstancedStaticMesh|UpdateInstanceTransform (Variables|Default|GetRailPiece) (- _index 1) (Spline|GetTransformatTime (Variables|Default|GetRCaterpillar) (* (+ (Math|Conversions|ToFloat(Integer) (- (Math|Integer|SelectInt 25 _index (== _index _returnvalue)) 25)) (Utilities|Select :Index (Variables|Default|GetRSelectIntegar) :Option%200 0.0 :Option%201 0.1 :Option%202 0.2 :Option%203 0.3 :Option%204 0.4 :Option%205 0.5 :Option%206 0.6 :Option%207 0.7 :Option%208 0.8 :Option%209 0.9)) (/ 1.0 (Math|Conversions|ToFloat(Integer) _lastindex))) "World" true false) true (== _index _returnvalue) false))
  (bind _result (Math|Integer|IncrementInt (Variables|Default|GetRSelectIntegar))
    (:%20%20
      (if (== _result 10)
        (Variables|Default|SetRSelectIntegar 0)))))

(event Custom|LCaterForward
  (bind _lastindex (Variables|Default|GetLastIndex))
  (for _index (range 1 _lastindex)
    (Components|InstancedStaticMesh|UpdateInstanceTransform (Variables|Default|GetRailPiece) (- _index 1) (Spline|GetTransformatTime (Variables|Default|GetLCaterpillar) (* (+ (Math|Conversions|ToFloat(Integer) (Math|Integer|SelectInt 0 _index (== _index _lastindex))) (Utilities|Select :Index (Variables|Default|GetLSelectIntegar) :Option%200 0.0 :Option%201 0.1 :Option%202 0.2 :Option%203 0.3 :Option%204 0.4 :Option%205 0.5 :Option%206 0.6 :Option%207 0.7 :Option%208 0.8 :Option%209 0.9)) (/ 1.0 (Math|Conversions|ToFloat(Integer) _lastindex))) "World" true false) true (== _index _lastindex) false))
  (bind _result (Math|Integer|IncrementInt (Variables|Default|GetLSelectIntegar))
    (:%20%20
      (if (== _result 10)
        (Variables|Default|SetLSelectIntegar 0)))))

(event Custom|LCaterBackward
  (bind _lastindex (Variables|Default|GetLastIndex))
  (for _index (range 1 _lastindex)
    (Components|InstancedStaticMesh|UpdateInstanceTransform (Variables|Default|GetRailPiece) (- _index 1) (Spline|GetTransformatTime (Variables|Default|GetLCaterpillar) (* (+ (Math|Conversions|ToFloat(Integer) (Math|Integer|SelectInt 25 _index (== _index _lastindex))) (* -1 (Utilities|Select :Index (Variables|Default|GetLSelectIntegar) :Option%200 0.0 :Option%201 0.1 :Option%202 0.2 :Option%203 0.3 :Option%204 0.4 :Option%205 0.5 :Option%206 0.6 :Option%207 0.7 :Option%208 0.8 :Option%209 0.9))) (/ 1.0 (Math|Conversions|ToFloat(Integer) _lastindex))) "World" true false) true (== _index _lastindex) false))
  (bind _result (Math|Integer|IncrementInt (Variables|Default|GetLSelectIntegar))
    (:%20%20
      (if (== _result 10)
        (Variables|Default|SetLSelectIntegar 0)))))

(event EventBeginPlay
  (bind _lastindex (Variables|Default|GetLastIndex))
  (bind _railpiece (Variables|Default|GetRailPiece))
  (Components|InstancedStaticMesh|ClearInstances _railpiece)
  (for _index (range 1 (* _lastindex 2))
    (Class|InstancedStaticMeshComponent|AddInstanceWorldSpace _railpiece (Spline|GetTransformatTime (select (>= _index 26) (Variables|Default|GetRCaterpillar) (Variables|Default|GetLCaterpillar)) (* (select (>= _index 26) (- _index 25) _index) (/ 1.0 (Math|Conversions|ToFloat(Integer) _lastindex))) "World" true true))))

(fn ConstructionScript)