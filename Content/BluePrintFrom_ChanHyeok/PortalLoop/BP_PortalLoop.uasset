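; Portal loop actor that carries MyCharacter_BP along an editable spline from one end to the other, then launches it upward.
; The construction script builds spline meshes between points and aligns Door1 and Door2 to the two ends.
; Box overlap triggers PortalJump, which disables character movement and chains latent MoveComponentTo steps along the spline at fixed distance intervals.
; At the end it restores walking, launches the character and resets its DoOnce guard.
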(event OnComponentBeginOverlap(Box)
  (params (OverlappedComponent :type Primitive%20Component%20Object%20Reference) (OtherActor :type Actor%20Object%20Reference) (OtherComp :type Primitive%20Component%20Object%20Reference) (OtherBodyIndex :type Integer) (bFromSweep :type Boolean) (SweepResult :type Hit%20Result%20Structure%20%28by%20ref%29))
  (bind _asmy_character_bp (Utilities|Casting|CastToMyCharacter_BP OtherActor))
  (CallFunction|PortalJump (Variables|Default|GetSpline)))

(event Custom|PortalJump
  (params (portal_spline :type Spline%20Component%20Object%20Reference) (directionNewParam :type Integer))
  ;[1 1 1] Portal Loop
  (Utilities|FlowControl|DoOnce false :!label _label
    (:Completed
      (Variables|Default|SetPortal%20Spline portal_spline)
      (Pawn|Components|CharacterMovement|SetMovementMode (Variables|/Script/Engine.Character|GetCharacterMovement (stale OnComponentBeginOverlap(Box) _asmy_character_bp)) "MOVE_None" 0)
      (bind _output_get (Variables|Default|SetPortal%20Distance 0.0))
      (if (< _output_get (Spline|GetSplineLength (Variables|Default|GetPortal%20Spline))) :!label _label_2
        (Components|MoveComponentTo (Variables|/Script/Engine.Character|GetCapsuleComponent (stale OnComponentBeginOverlap(Box) _asmy_character_bp)) (.location (Spline|GetTransformatDistanceAlongSpline (Variables|Default|GetPortal%20Spline) (Variables|Default|GetPortal%20Distance) "World" false)) "0, 0, 0" false false 0.1 false)
        (Variables|Default|SetPortal%20Distance (+ (Variables|Default|GetPortal%20Distance) 3e+02))
        (goto _label_2)
        (else
          (Variables|Default|SetPortal%20Distance (Spline|GetSplineLength (Variables|Default|GetPortal%20Spline)))
          (Components|MoveComponentTo (Variables|/Script/Engine.Character|GetCapsuleComponent (stale OnComponentBeginOverlap(Box) _asmy_character_bp)) (.location (Spline|GetTransformatDistanceAlongSpline (Variables|Default|GetPortal%20Spline) (Variables|Default|GetPortal%20Distance) "World" false)) "0, 0, 0" false false 0.2 false)
          (Pawn|Components|CharacterMovement|SetMovementMode (Variables|/Script/Engine.Character|GetCharacterMovement (stale OnComponentBeginOverlap(Box) _asmy_character_bp)) "MOVE_Walking" 0)
          (Components|MoveComponentTo (Variables|/Script/Engine.Character|GetCapsuleComponent (stale OnComponentBeginOverlap(Box) _asmy_character_bp)) (Transformation|GetWorldLocation (Variables|/Script/Engine.Character|GetCapsuleComponent (stale OnComponentBeginOverlap(Box) _asmy_character_bp))) (Variables|/Script/Engine.SceneComponent|GetRelativeRotation (Variables|/Script/Engine.Character|GetCapsuleComponent (stale OnComponentBeginOverlap(Box) _asmy_character_bp))) false false 0.1 false)
          (Character|LaunchCharacter (stale OnComponentBeginOverlap(Box) _asmy_character_bp) "0, 0,1000.000000" false false)
          (goto _label Reset))))))

(event EventBeginPlay)

(event Collision|EventActorBeginOverlap
  (params (OtherActor :type Actor%20Object%20Reference)))

(event EventTick
  (params (DeltaSeconds :type Float%20%28single-precision%29)))

(fn ConstructionScript
  (bind _spline (Variables|Default|GetSpline))
  (bind _spline_2 (Variables|Default|GetSpline))
  (bind _returnvalue (Spline|GetTransformatSplinePoint _spline_2 0 "Local" false))
  (bind _returnvalue_2 (Spline|GetNumberOfSplinePoints _spline_2))
  (bind _returnvalue_3 (- _returnvalue_2 1))
  (bind _returnvalue_4 (Spline|GetTransformatSplinePoint _spline_2 _returnvalue_3 "Local" false))
  ;[1 1 1] Portal loop
  (for _index (range 0 (- (Spline|GetNumberOfSplinePoints _spline) 2))
    (bind _returnvalue_5 (AddComponent|AddSplineMeshComponent false))
    (SplineMesh|SetStartandEnd _returnvalue_5 (.Location (Spline|GetLocationandTangentatSplinePoint _spline _index "Local")) (.Tangent (Spline|GetLocationandTangentatSplinePoint _spline _index "Local")) (.Location (Spline|GetLocationandTangentatSplinePoint _spline (+ _index 1) "Local")) (.Tangent (Spline|GetLocationandTangentatSplinePoint _spline (+ _index 1) "Local")) true :!class /Script/Engine.SplineMeshComponent)
    (Transformation|SetRelativeLocationAndRotation (Variables|Default|Getdoor1) (.location _returnvalue) (Math|Rotator|MakeRotator (.roll (.rotation _returnvalue)) (+ (.pitch (.rotation _returnvalue)) 9e+01) (.yaw (.rotation _returnvalue))) false false)
    (Transformation|SetRelativeLocationAndRotation (Variables|Default|Getdoor2) (.location _returnvalue_4) (Math|Rotator|MakeRotator (.roll (.rotation _returnvalue_4)) (+ (.pitch (.rotation _returnvalue_4)) 9e+01) (.yaw (.rotation _returnvalue_4))) false false)))

(fn GetClientController
  (return 0))