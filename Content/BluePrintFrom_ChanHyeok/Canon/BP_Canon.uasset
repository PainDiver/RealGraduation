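; Rideable, networked cannon that fires bullets automatically while unoccupied and on the Attack input when possessed.
; Riding attaches the rider to the seat through a server-to-multicast event chain.
; A looping timer fires straight along the arrow on authority; held Attack repeats shots with an upward tilt, and a release delay limits refiring.
; Both fire paths spawn BP_Bullet and call a multicast explosion effect at the muzzle.
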(event Custom|ShootServer
  (bind _self self)
  (bind _arrow (Variables|Default|GetArrow))
  (Game|SpawnActorfromClass "/Game/BluePrintFrom_ChanHyeok/Canon/Bullet/BP_Bullet.BP_Bullet_C" (Math|Transform|MakeTransform (Transformation|GetWorldLocation _arrow) (Transformation|GetWorldRotation _arrow) "1,1,1") "Undefined" _self _self)
  (CallFunction|EffectMulti))

(event Custom|ShootServerInPossess
  (bind _self self)
  (Game|SpawnActorfromClass "/Game/BluePrintFrom_ChanHyeok/Canon/Bullet/BP_Bullet.BP_Bullet_C" (Math|Transform|MakeTransform (Transformation|GetWorldLocation (Variables|Default|GetArrow)) (Math|Conversions|RotationFromXVector (+ (* (Math|Vector|GetForwardVector (Variables|Default|GetArrow)) 2e+03) "0, 0,300.000000")) "1,1,1") "Undefined" _self _self)
  (CallFunction|EffectMulti))

(event Custom|AttachActorServer
  (CallFunction|AttachActorMulti))

(event Custom|AttachActorMulti
  (bind _rider (Variables|Default|GetRider))
  (Utilities|IsValid _rider
    (:Is%20Valid
      (Transformation|AttachComponentToComponent _rider (Variables|Default|GetRidingSpot) (Variables|Default|GetSocketName) "SnapToTarget" "SnapToTarget" "KeepWorld" false))))

(event Custom|EffectMulti
  (Effects|SpawnEmitteratLocation "/Game/StarterContent/Particles/P_Explosion.P_Explosion" (Transformation|GetWorldLocation (Variables|Default|GetArrow))))

(event Custom|Shoot
  (Networking|SwitchHasAuthority
    (:Authority
      (if (not (Variables|Default|GetBeingUsed))
        (CallFunction|ShootServer)))))

(event EventBeginPlay
  (Utilities|Time|SetTimerbyEvent (delegate Custom|Shoot) 0.7 true 0.7)
  (|CallParentFunction))

(event EventRide
  (params (DelegateCaller :type Actor%20Object%20Reference))
  (|CallParentFunction DelegateCaller)
  (CallFunction|AttachActorServer))

(event EventTick
  (params (DeltaSeconds :type Float%20%28single-precision%29)))

(event EventSaveData
  (|CallParentFunction))

(event Input|ActionEvents|InputActionAttack
  (params (Key :type Key%20Structure :default "None"))
  (:Pressed
    (if (not (Variables|Default|GetIsShooting))
      (Variables|Default|SetIsShooting true)
      (CallFunction|ShootServerinPossess)
      (bind _returnvalue (Utilities|Time|SetTimerbyEvent (delegate Custom|ShootServerInPossess) 0.7 true))
      (Variables|Default|SetTimerHandle _returnvalue)))
  (:Released
    (Utilities|Time|ClearandInvalidateTimerbyHandle (Variables|Default|GetTimerHandle))
    (Utilities|FlowControl|Delay 0.7)
    (Variables|Default|SetIsShooting false)))

(fn ConstructionScript)