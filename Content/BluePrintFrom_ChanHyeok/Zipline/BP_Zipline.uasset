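; Zipline actor that carries a player character from its start point to its end point when activated.
; A cable is strung between the two tops, and overlapping the start sphere stores the travel direction.
; Activation disables rider input, switches movement to Flying with a parkour sledging flag, and slides the capsule via MoveComponentTo in distance-scaled time.
; On arrival it restores input, sets Falling and clears the flag.
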(event Custom|SetDirFromStart
  (params (OverlappedComponent :type Primitive%20Component%20Object%20Reference) (OtherActor :type Actor%20Object%20Reference) (OtherComp :type Primitive%20Component%20Object%20Reference) (OtherBodyIndex :type Integer) (bFromSweep :type Boolean) (SweepResult :type Hit%20Result%20Structure%20%28by%20ref%29))
  (CallFunction|SetDirection (Transformation|GetWorldLocation (Variables|Default|GetStart1)) (Transformation|GetWorldLocation (Variables|Default|GetEnd1)))
  (Development|PrintString "Hello"))

(event Custom|Server%20Zipline
  (bind _zipstartposition (Variables|Default|GetZipStartPosition))
  (bind _zipendposition (Variables|Default|GetZipEndPosition))
  (bind _rider (Variables|Default|GetRider))
  (bind _returnvalue (+ _zipendposition "0, 0,-90.000000"))
  (CallFunction|DisableInputMulti)
  (Variables|/Script/MyProject4.MyCharacterParkourComponent|Set_bIsledging (Variables|/Script/MyProject4.MyCharacter|Get_parkourComponent _rider) true)
  (Pawn|Components|CharacterMovement|SetMovementMode (Variables|/Script/Engine.Character|GetCharacterMovement _rider) "MOVE_Flying" 0)
  (Components|MoveComponentTo (Variables|/Script/Engine.Character|GetCapsuleComponent (Variables|Default|GetRider)) (+ _zipstartposition "0, 0,-90.000000") (Math|Rotator|FindLookatRotation _zipstartposition (Variables|Default|GetZipEndPosition)) false true 0.1 false)
  (Components|MoveComponentTo (Variables|/Script/Engine.Character|GetCapsuleComponent (Variables|Default|GetRider)) _returnvalue (Transformation|GetActorRotation) false true (/ (Math|Vector|Distance(Vector) _returnvalue (Variables|Default|GetZipStartPosition)) 1e+03) false)
  (CallFunction|EnableInputMulti)
  (Pawn|Components|CharacterMovement|SetMovementMode (Variables|/Script/Engine.Character|GetCharacterMovement (Variables|Default|GetRider)) "MOVE_Falling" 0)
  (Variables|/Script/MyProject4.MyCharacterParkourComponent|Set_bIsledging (Variables|/Script/MyProject4.MyCharacter|Get_parkourComponent (Variables|Default|GetRider)) false))

(event Custom|EnableInputMulti
  (bind _rider (Variables|Default|GetRider))
  (Utilities|IsValid _rider
    (:Is%20Valid
      (Input|EnableInput _rider 0))))

(event Custom|DisableInputMulti
  (bind _rider (Variables|Default|GetRider))
  (Utilities|IsValid _rider
    (:Is%20Valid
      (Input|DisableInput _rider 0))))

(event Custom|SetDirection
  (params (start%20postion :type Vector) (end%20postion :type Vector))
  (Variables|Default|SetZip%20Enable false)
  (Variables|Default|SetZipStartPosition start%20postion)
  (Variables|Default|SetZipEndPosition end%20postion))

(event EventBeginPlay
  (|CallParentFunction)
  (Utilities|InitCable)
  (Collision|BindEventtoOnComponentBeginOverlap (Variables|Default|GetSphere1) (delegate Custom|SetDirFromStart)))

(event Collision|EventActorBeginOverlap
  (params (OtherActor :type Actor%20Object%20Reference)))

(event EventTick
  (params (DeltaSeconds :type Float%20%28single-precision%29)))

(event EventActivate
  (params (DelegateCaller :type Actor%20Object%20Reference))
  (|CallParentFunction DelegateCaller)
  (Variables|Default|SetRider (.AsMy%20Character%20BP (Utilities|Casting|CastToMyCharacter_BP DelegateCaller)))
  (CallFunction|ServerZipline))

(fn ConstructionScript
  (Utilities|InitCable))