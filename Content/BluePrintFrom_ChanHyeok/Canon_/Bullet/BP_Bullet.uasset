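; BP_Bullet is a cannon bullet actor that explodes on overlap with anything except its owner, then destroys itself.
; An overlapped MyCharacter_BP is launched through ServerHit along fixed world +X with slight lift, regardless of bullet direction.
; Both hit paths call EffectMulti for the explosion particle and sound, the names suggesting server and multicast RPCs.
; The Hit function, BeginPlay and Tick are empty.
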(event Custom|ServerHit
  (Utilities|IsValid (stale Collision|EventActorBeginOverlap _asmy_character_bp)
    (:Is%20Valid
      (Character|LaunchCharacter (stale Collision|EventActorBeginOverlap _asmy_character_bp) "1500.000000,0.000000,100.000000" false true)
      (CallFunction|EffectMulti))))

(event Custom|EffectMulti
  (bind _returnvalue (Transformation|GetActorLocation))
  (Effects|SpawnEmitteratLocation "/Game/StarterContent/Particles/P_Explosion.P_Explosion" _returnvalue "0, 0, 0" "3.000000,3.000000,3.000000")
  (Audio|PlaySoundatLocation "/Game/StarterContent/Audio/Explosion_Cue.Explosion_Cue" _returnvalue "0, 0, 0" 0.5 0.5 0.0 0 0 0))

(event EventBeginPlay)

(event Collision|EventActorBeginOverlap
  (params (OtherActor :type Actor%20Object%20Reference))
  (if (not (== OtherActor (Components|GetOwner)))
    (bind _asmy_character_bp (Utilities|Casting|CastToMyCharacter_BP OtherActor)
      (:then
        (CallFunction|ServerHit)
        (Actor|DestroyActor))
      (:CastFailed
        (CallFunction|EffectMulti)
        (Actor|DestroyActor)))))

(event EventTick
  (params (DeltaSeconds :type Float%20%28single-precision%29)))

(fn ConstructionScript)

(fn Hit
  (params (Target :type My%20Character%20BP%20Object%20Reference)))