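; Game mode for the ready room lobby, which runs the pre-match countdown on Steam dedicated servers.
; On a dedicated server it registers the session, reports player joins and leaves, and exits when a periodic check finds the room empty.
; A looping timer counts down while players are present, publishes through GameState, and flags the session started near the end.
; At zero it destroys pawns, hides player widgets and ServerTravels to the matching gameplay map.
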(event Custom|DediCheck
  (bind _returnvalue (Class|MyGameInstance|DediCheck (.AsMy%20Game%20Instance%20BP (Utilities|Casting|CastToMyGameInstance_BP (Game|GetGameInstance)))))
  (if _returnvalue
    (Variables|Default|SetdedicatedServer true)
    (Development|PrintString "Dedi")
    (else
      (Variables|Default|SetdedicatedServer false)
      (Development|PrintString "NotDedi"))))

(event Custom|NotifyAllStopWidget
  (CallFunction|NotifyAllStopWidgetMulti))

(event Custom|Counter
  (bind _returnvalue (Game|GetGameState))
  (bind _returnvalue_2 (Game|GetGameState))
  (bind _returnvalue_3 (Game|GetGameInstance))
  (bind _asready_room_game_state_base_bp (Utilities|Casting|CastToReadyRoomGameStateBase_BP _returnvalue))
  (bind _asready_room_game_state_base_bp_2 (Utilities|Casting|CastToReadyRoomGameStateBase_BP _returnvalue_2))
  (bind _asmy_game_instance_bp (Utilities|Casting|CastToMyGameInstance_BP _returnvalue_3))
  (if (>= (Utilities|Array|Length (Variables|/Script/Engine.GameStateBase|GetPlayerArray (.AsReady%20Room%20Game%20State%20Base%20BP (Utilities|Casting|CastToReadyRoomGameStateBase_BP (Game|GetGameState))))) 1)
    (bind _output_get (Variables|Default|SetStartCount (- (Variables|Default|GetStartCount) 1)))
    (Utilities|IsValid _asready_room_game_state_base_bp_2
      (:Is%20Valid
        (Variables|/Game/ReadyRoomMap/ReadyRoomGameStateBase_BP.ReadyRoomGameStateBase_BP_C|SetStartCountFromServer _asready_room_game_state_base_bp_2 _output_get)
        (if (>= 15 (Variables|Default|GetStartCount))
          (if (Variables|Default|GetUpdatePending)
            _
            (else
              (Variables|Default|SetUpdatePending true)
              (Class|MyGameInstance|UpdateDedicatedServerState _asmy_game_instance_bp (Class|AdvancedSessionsLibrary|GetCurrentSessionIDasString) true)))
          (if (>= 0 (Variables|Default|GetStartCount))
            (Utilities|Time|ClearandInvalidateTimerbyHandle (Variables|Default|GetTimer))
            (Utilities|IsValid _asmy_game_instance_bp
              (:Is%20Valid
                (Utilities|FlowControl|Delay 3.0)
                (bind _outactors (Actor|GetAllActorsOfClass "/Script/Engine.Pawn"))
                (bind _array_element (Utilities|Array|ForEachLoopwithBreak _outactors)
                  (:LoopBody
                    (Actor|DestroyActor _array_element)
                    (Variables|/Script/MyProject4.MyGameInstance|Set_gameEnterClosed _asmy_game_instance_bp true)
                    (Utilities|IsValid _asready_room_game_state_base_bp
                      (:Is%20Valid
                        (bind _returnvalue_4 (Class|ReadyRoomGameStateBase|GetNumberOfUser _asready_room_game_state_base_bp))
                        (Variables|/Script/MyProject4.MyGameInstance|Set_numOfPlayerInCurrentSession _asmy_game_instance_bp _returnvalue_4)
                        (CallFunction|NotifyAllStopWidget)
                        (bind _returnvalue_5 (Class|MyGameInstance|GetWorldName (.AsMy%20Game%20Instance%20BP (Utilities|Casting|CastToMyGameInstance_BP (Game|GetGameInstance)))))
                        (switch string _returnvalue_5
                          (:ReadyMap
                            (Development|ExecuteConsoleCommand "ServerTravel/Game/map/simplemap?game=/Game/BluePrintFrom_Me/MyMyProject4GameModeBase_BP.MyMyProject4GameModeBase_BP_C" 0))
                          (:SpaceStationReadyMap
                            (Development|ExecuteConsoleCommand "ServerTravel/Game/map/SpaceMap?game=/Game/BluePrintFrom_Me/MyMyProject4GameModeBase_BP.MyMyProject4GameModeBase_BP_C" 0)))))))))))))))

(event Custom|Exit
  (bind _returnvalue (Game|GetGameState))
  (bind _returnvalue_2 (Game|GetGameInstance))
  (bind _asready_room_game_state_base_bp (Utilities|Casting|CastToReadyRoomGameStateBase_BP _returnvalue))
  (bind _asmy_game_instance_bp (Utilities|Casting|CastToMyGameInstance_BP _returnvalue_2))
  (bind _playerarray (Variables|/Script/Engine.GameStateBase|GetPlayerArray _asready_room_game_state_base_bp))
  (bind _returnvalue_3 (Utilities|Array|Length _playerarray))
  (Utilities|IsValid _asready_room_game_state_base_bp
    (:Is%20Valid
      (Development|PrintString (Utilities|String|Append (Utilities|String|MakeLiteralString "Person Check") (Utilities|String|ToString(Integer) _returnvalue_3)))
      (if (== _returnvalue_3 0)
        (Class|MyGameInstance|LogOutDediServer _asmy_game_instance_bp (Class|AdvancedSessionsLibrary|GetCurrentSessionIDasString))
        (Utilities|Time|ClearandInvalidateTimerbyHandle (Variables|Default|GetTimer))
        (Utilities|Time|ClearandInvalidateTimerbyHandle (Variables|Default|GetTimer2))
        (Class|MyGameInstance|RequestExit _asmy_game_instance_bp false)))))

(event Custom|NotifyAllStopWidgetMulti
  (bind _asready_room_game_state_base_bp (Utilities|Casting|CastToReadyRoomGameStateBase_BP (Game|GetGameState)))
  (Class|ReadyRoomGameStateBase|FindAllPlayerControllerHideAllWidget _asready_room_game_state_base_bp))

(event EventBeginPlay
  (bind _returnvalue (Class|MyGameInstance|GetWorldName (.AsMy%20Game%20Instance%20BP (Utilities|Casting|CastToMyGameInstance_BP (Game|GetGameInstance)))))
  (Development|PrintString _returnvalue)
  (CallFunction|DediCheck)
  (Utilities|FlowControl|Delay 1.0)
  (if (Variables|Default|GetdedicatedServer)
    (Utilities|FlowControl|Delay 1.0)
    (Class|MyGameInstance|WriteDedicatedServerInfo (.AsMy%20Game%20Instance%20BP (Utilities|Casting|CastToMyGameInstance_BP (Game|GetGameInstance))) (Class|AdvancedSessionsLibrary|GetCurrentSessionIDasString))
    (Utilities|FlowControl|Delay 1.0)
    (Class|MyGameInstance|UpdateDedicatedServerState (.AsMy%20Game%20Instance%20BP (Utilities|Casting|CastToMyGameInstance_BP (Game|GetGameInstance))) (Class|AdvancedSessionsLibrary|GetCurrentSessionIDasString) false)
    (Variables|/Game/ReadyRoomMap/ReadyRoomGameStateBase_BP.ReadyRoomGameStateBase_BP_C|SetIsdedicatedServer (.AsReady%20Room%20Game%20State%20Base%20BP (Utilities|Casting|CastToReadyRoomGameStateBase_BP (Game|GetGameState))) true)
    (bind _returnvalue_2 (Utilities|Time|SetTimerbyEvent (delegate Custom|Counter) 1.0 true))
    (Variables|Default|SetTimer _returnvalue_2)
    (bind _returnvalue_3 (Utilities|Time|SetTimerbyEvent (delegate Custom|Exit) 6e+01 true))
    (Variables|Default|SetTimer2 _returnvalue_3)))

(event EventOnLogout
  (params (ExitingController :type Controller%20Object%20Reference))
  (if (Class|KismetSystemLibrary|IsPackagedforDistribution)
    (if (Networking|IsDedicatedServer)
      (Class|MyGameInstance|LinkDedicatedServerInfo (.AsMy%20Game%20Instance%20BP (Utilities|Casting|CastToMyGameInstance_BP (Game|GetGameInstance))) (Class|AdvancedSessionsLibrary|GetCurrentSessionIDasString) false))))

(event EventPostLogin
  (params (NewPlayer :type Player%20Controller%20Object%20Reference))
  (if (Networking|IsDedicatedServer)
    (Class|MyGameInstance|LinkDedicatedServerInfo (.AsMy%20Game%20Instance%20BP (Utilities|Casting|CastToMyGameInstance_BP (Game|GetGameInstance))) (Class|AdvancedSessionsLibrary|GetCurrentSessionIDasString) true)))

(fn ConstructionScript)