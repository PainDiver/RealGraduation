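; Player controller for the ready room map that sets up the local player's pre-game UI.
; On BeginPlay it asks the game instance whether the session runs on a dedicated server, using short delays around the check.
; Dedicated sessions show a start counter widget, while others show a next map widget kept as MapInfoUI.
; Events also store the player's ready state and selected map.
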(event Custom|DediCheck
  (bind _returnvalue (Class|MyGameInstance|DediCheck (.AsMy%20Game%20Instance%20BP (Utilities|Casting|CastToMyGameInstance_BP (Game|GetGameInstance)))))
  (if _returnvalue
    (Variables|Default|SetdedicatedServer true)
    (Development|PrintString "Dedi")
    (else
      (Variables|Default|SetdedicatedServer false)
      (Development|PrintString "NotDedi"))))

(event Custom|SetReady
  (params (NewParam :type Boolean))
  (Variables|Default|SetIsReady NewParam))

(event Custom|SelectMap
  (params (NewParam :type String))
  (Variables|Default|SetSetMap NewParam))

(event EventBeginPlay
  (bind _returnvalue (Game|GetPlayerController 0))
  (if (Pawn|IsLocalController)
    (Utilities|FlowControl|Delay 2.0)
    (CallFunction|DediCheck)
    (Utilities|FlowControl|Delay 1.0)
    (if (Variables|Default|GetDedicatedServer)
      (bind _returnvalue_2 (UserInterface|CreateWidget "/Game/HUD/StartCounter_UI.StartCounter_UI_C" _returnvalue))
      (Utilities|IsValid _returnvalue_2
        (:Is%20Valid
          (UserInterface|Viewport|AddtoViewport _returnvalue_2 1)))
      (else
        (bind _returnvalue_3 (UserInterface|CreateWidget "/Game/HUD/NextMap_UI.NextMap_UI_C" _returnvalue))
        (bind _output_get (Variables|Default|SetMapInfoUI _returnvalue_3))
        (Utilities|IsValid _output_get
          (:Is%20Valid
            (UserInterface|Viewport|AddtoViewport _returnvalue_3 0)))))))

(event EventTick
  (params (DeltaSeconds :type Float%20%28single-precision%29)))

(fn ConstructionScript)