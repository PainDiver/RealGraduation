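; Title screen controller for the title map that shows a press-any-key prompt before revealing the title UI.
; On BeginPlay it applies a hardware benchmark to the graphics settings, hides the cursor and adds the main title, title UI and prompt widgets, with the main title layered behind.
; The first key press, gated by a one-shot flag, shows the cursor and title UI, hides the prompt and fades the background poster.
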(event EventBeginPlay
  (bind _returnvalue (Settings|GetGameUserSettings))
  (Class|GameUserSettings|RunHardwareBenchmark _returnvalue 10 1.0 1.0)
  (Class|GameUserSettings|ApplyHardwareBenchmarkResults _returnvalue)
  (Variables|Default|Setinitial false)
  (Variables|Default|SetbShowMouseCursor false)
  (bind _asplayer_controller (Utilities|Casting|CastToPlayerController (Pawn|GetController (Game|Player|GetPlayerPawn 0))))
  (Utilities|FlowControl|Sequence
    (:then_0
      (bind _returnvalue_2 (UserInterface|CreateWidget "/Game/TitleMap/MainTitle_UI.MainTitle_UI_C" _asplayer_controller))
      (UserInterface|Viewport|AddtoViewport _returnvalue_2 -50))
    (:then_1
      (bind _returnvalue_3 (UserInterface|CreateWidget "/Game/HUD/TitleUI.TitleUI_C" _asplayer_controller))
      (UserInterface|Viewport|AddtoViewport _returnvalue_3 0))
    (:then_2
      (bind _returnvalue_4 (UserInterface|CreateWidget "/Game/HUD/PressAnyKey_UI.PressAnyKey_UI_C" _asplayer_controller))
      (UserInterface|Viewport|AddtoViewport _returnvalue_4 0))))

(event EventTick
  (params (DeltaSeconds :type Float%20%28single-precision%29)))

(event Input|KeyboardEvents|AnyKey
  (params (Key :type Key%20Structure :default "None"))
  (:Pressed
    (if (not (Variables|Default|Getinitial))
      (Variables|Default|SetKeyInput true)
      (Variables|Default|SetbShowMouseCursor true)
      (Widget|SetVisibility (stale EventBeginPlay _returnvalue_3) "Visible")
      (Widget|SetVisibility (stale EventBeginPlay _returnvalue_4) "Hidden")
      (Class|Image|SetOpacity (Variables|/Game/TitleMap/MainTitle_UI.MainTitle_UI_C|GetPoster (stale EventBeginPlay _returnvalue_2)) 0.3)
      (Variables|Default|Setinitial true))))

(fn ConstructionScript)