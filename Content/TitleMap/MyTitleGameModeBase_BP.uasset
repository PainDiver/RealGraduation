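; Title map game mode that uses a save slot as a persistent flag for a master server.
; On BeginPlay, the server checks the MasterServer slot: if a save exists, it issues a ServerTravel console command to ReadyMap as a listen server.
; Otherwise it writes a new ServerSave with IsMasterServer set and stays on the map.
; When player controller 0 logs out, it deletes that slot.
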(event EventBeginPlay
  (if (Networking|IsServer)
    (bind _returnvalue (SaveGame|LoadGamefromSlot "MasterServer"))
    (Utilities|IsValid _returnvalue
      (:Is%20Valid
        (Development|ExecuteConsoleCommand "ServerTravel/Game/map/ReadyMap?listen" 0))
      (:Is%20Not%20Valid
        (bind _returnvalue_2 (SaveGame|CreateSaveGameObject "/Game/TitleMap/ServerSave.ServerSave_C"))
        (Variables|/Game/TitleMap/ServerSave.ServerSave_C|SetIsMasterServer _returnvalue_2 true)
        (SaveGame|SaveGametoSlot _returnvalue_2 "MasterServer")))))

(event EventTick
  (params (DeltaSeconds :type Float%20%28single-precision%29)))

(event EventOnLogout
  (params (ExitingController :type Controller%20Object%20Reference))
  (if (== ExitingController (Game|GetPlayerController 0))
    (SaveGame|DeleteGameinSlot "MasterServer")))

(fn ConstructionScript)