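; Player controller Blueprint for the score map that shuts down input and UI a fixed delay after play begins.
; After the parent BeginPlay and the delay, it checks that player controller 0 is valid and local, then disables its input.
; It then casts that controller to its own class to clear two timer handles, and removes all widgets.
; Tick and the construction script are empty.
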(event EventBeginPlay
  (bind _returnvalue (Game|GetPlayerController 0))
  (bind _asmy_score_map_player_controller_bp (Utilities|Casting|CastToMyScoreMapPlayerController_BP _returnvalue))
  (|CallParentFunction)
  (Utilities|FlowControl|Delay 13.0)
  (Utilities|IsValid _returnvalue
    (:Is%20Valid
      (if (Pawn|IsLocalPlayerController _returnvalue)
        (Input|DisableInput _returnvalue)
        (Utilities|Time|ClearandInvalidateTimerbyHandle (Variables|/Script/MyProject4.MyScoreMapPlayerController|Get_timerHandle _asmy_score_map_player_controller_bp))
        (Utilities|Time|ClearandInvalidateTimerbyHandle (Variables|/Script/MyProject4.MyScoreMapPlayerController|Get_timerHandle2 _asmy_score_map_player_controller_bp))
        (Viewport|RemoveAllWidgets)))))

(event EventTick
  (params (DeltaSeconds :type Float%20%28single-precision%29)))

(fn ConstructionScript)